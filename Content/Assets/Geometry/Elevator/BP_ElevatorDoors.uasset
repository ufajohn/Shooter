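; Elevator door Blueprint that slides a left and right door apart to open and together to close.
; The OpenDoors and CloseDoors events move both door components in opposite directions along relative Y with eased, timed MoveComponentTo calls.
; Each move is a fixed offset from the door's current position, with no open/closed state check, and OpenDoors ignores its Floor input.
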(event `CloseDoors`
  (bind _returnvalue_location (`KismetMathLibrary.BreakTransform` (`SceneComponent.GetRelativeTransform` (`self.R_Door`))))
  (bind _returnvalue_location_2 (`KismetMathLibrary.BreakTransform` (`SceneComponent.GetRelativeTransform` (`self.L_Door`))))
  ;[1 1 1] Close Doors
  (`|ExecutionSequence`
    (:`then_0`
      (`KismetSystemLibrary.MoveComponentTo` (`self.L_Door`) (`KismetMathLibrary.MakeVector` (.x _returnvalue_location_2) (+ (.y _returnvalue_location_2) 63.0) (.z _returnvalue_location_2)) (struct) true true 3.0))
    (:`then_1`
      (`KismetSystemLibrary.MoveComponentTo` (`self.R_Door`) (`KismetMathLibrary.MakeVector` (.x _returnvalue_location) (- (.y _returnvalue_location) 63.0) (.z _returnvalue_location)) (struct) true true 3.0))))

(event `OpenDoors`
  (params (Floor :type Integer))
  (bind _returnvalue_location (`KismetMathLibrary.BreakTransform` (`SceneComponent.GetRelativeTransform` (`self.L_Door`))))
  (bind _returnvalue_location_2 (`KismetMathLibrary.BreakTransform` (`SceneComponent.GetRelativeTransform` (`self.R_Door`))))
  ;[1 1 1] Open Doors
  (`|ExecutionSequence`
    (:`then_0`
      (`KismetSystemLibrary.MoveComponentTo` (`self.L_Door`) (`KismetMathLibrary.MakeVector` (.x _returnvalue_location) (- (.y _returnvalue_location) 63.0) (.z _returnvalue_location)) (struct) true true 3.0))
    (:`then_1`
      (`KismetSystemLibrary.MoveComponentTo` (`self.R_Door`) (`KismetMathLibrary.MakeVector` (.x _returnvalue_location_2) (+ (.y _returnvalue_location_2) 63.0) (.z _returnvalue_location_2)) (struct) true true 3.0))))

(fn `UserConstructionScript`
  (locals (Increment :type Integer) (NewLocalVar_0 :type "SceneComponent Object Reference")))