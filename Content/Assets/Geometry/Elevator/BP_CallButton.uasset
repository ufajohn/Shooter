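; Elevator call button that a character interacts with to call its linked Elevator, passing itself and the hit to UpDown.
; The construction script derives CallFloor from the button's world height, measured against the elevator's first-floor height and floor spacing.
; On BeginPlay it binds to the elevator's button-activate and downtime-deactivate events, which swap the mesh's emissive material instance to show the button's state.
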(event `self.ReceiveBeginPlay`
  (bind _elevator (`self.Elevator`)
    (:`then`
      (add `/Game/Assets/Geometry/Elevator/BP_elevator.ButtonActivate` _elevator (delegate `ButtonActivateEvent`))
      (add `/Game/Assets/Geometry/Elevator/BP_elevator.ElevatorDeactivateOnDowntime` (`self.Elevator`) (delegate `ElevatorDeactivate_Event_0`)))
    (:`else`)))

(event `ElevatorDeactivate_Event_0`
  (`PrimitiveComponent.SetMaterial` (`self.StaticMeshComponent`) 0 "/Game/Assets/Geometry/Elevator/BaseEmissive_Inst.BaseEmissive_Inst"))

(event `ButtonActivateEvent`
  (`PrimitiveComponent.SetMaterial` (`self.StaticMeshComponent`) 0 "/Game/Assets/Geometry/Elevator/BaseEmissive_Inst1.BaseEmissive_Inst1"))

(fn `Interact`
  (params (Character :type "/Game/Blueprints/Characters/BP_PlayerCharacter Object Reference") (Hit :type "HitResult Structure"))
  (returns (Success :type Boolean))
  (`/Game/Assets/Geometry/Elevator/BP_elevator.UpDown` (`self.Elevator`) Hit self)
  (return true))

(fn `UserConstructionScript`
  (locals (Increment :type Integer :default 1))
  (bind _elevator (`self.Elevator`))
  (bind _z (.z (`SceneComponent.K2_GetComponentLocation` (`self.StaticMeshComponent`))))
  (bind _heightfirstfloor (`/Game/Assets/Geometry/Elevator/BP_elevator.GetHeightFirstFloor` _elevator (`/Game/Assets/Geometry/Elevator/BP_elevator.Building` _elevator)))
  (for _index (range (+ (`/Game/Assets/Geometry/Elevator/BP_elevator.NumberOfFloors` _elevator) 1))
    (if (and (> _z _heightfirstfloor) (< _z (+ _heightfirstfloor (`KismetMathLibrary.Conv_IntToDouble` (* (`/Game/Assets/Geometry/Elevator/BP_elevator.HeightFloor` _elevator) (`self.Increment`))))))
      (break)
      (else
        (`/Engine/EditorBlueprintResources/StandardMacros.IncrementInt` (`self.Increment`)))))
  (set `self.CallFloor` (+ _index 1)))