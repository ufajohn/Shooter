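; Interactable elevator that moves a cabin between a building's floors from a call button or in-cabin floor buttons, with a stop button to halt it.
; Floor buttons come from CommandBar's children, and the current floor derives from cabin height.
; MoveComponentTo eases the cabin to its target, then slides its doors alongside the overlapping BP_ElevatorDoors and auto-closes them.
; Dispatchers sequence travel, doors, sounds, button glow and idle shutdown, deferring requests until doors close.
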(event `self.ReceiveBeginPlay`
  (add `self.ElevatorActivate` (delegate `ElevatorActivate_Event`))
  (add `self.ElevatorDeactivate` (delegate `ElevatorDeactivate_Event`)))

(event `ElevatorActivate_Event`
  (`AudioComponent.Play` (`self.лифт`) 0.0))

(event `ElevatorDeactivate_Event`
  (`AudioComponent.Stop` (`self.лифт`))
  (for _array_element (`self.FloorsArray`)
    (`PrimitiveComponent.SetMaterial` (cast `StaticMeshComponent` _array_element :!pure true) 1 "/Game/Assets/Geometry/Elevator/BaseEmissive_Inst.BaseEmissive_Inst")))

(event `Event1`
  (bind _staticmeshcomponent (`self.StaticMeshComponent`))
  (bind _returnvalue (+ (`self.HeightFirstFloor`) (`KismetMathLibrary.Conv_IntToDouble` (- (* (- (`self.CurrentFloor`) 1) (`self.HeightFloor`)) 20))))
  ;[1 1 1] Main Logic
  (if true
    (goto _label_4 :!via `Stop`)
    (else
      (`/Engine/EditorBlueprintResources/StandardMacros.DoOnce` (`self.StopButton`) :!label _label
        (:`Completed`
          (bind _output_get (set `self.NewFloor` (`/Game/Assets/Geometry/Elevator/BP_CallButton.CallFloor` (stale `UpDown` CallButton)) :!label _label_2))
          (if (!= _output_get (`self.GetCurrentFloor`))
            (set `self.Activate` true :!label _label_3)
            (`PrimitiveComponent.SetMaterial` (`self.stop`) 1 "/Game/Assets/Geometry/Elevator/BaseEmissive_Inst.BaseEmissive_Inst")
            (`self.ElevatorActivate`)
            (`KismetSystemLibrary.MoveComponentTo` (`self.StaticMeshComponent`) (`KismetMathLibrary.MakeVector` (.x (`SceneComponent.K2_GetComponentLocation` _staticmeshcomponent)) (.y (`SceneComponent.K2_GetComponentLocation` _staticmeshcomponent)) (+ (- (`self.HeightFirstFloor`) 20.0) (`KismetMathLibrary.Conv_IntToDouble` (* (`self.HeightFloor`) (- (`self.NewFloor`) 1))))) (`SceneComponent.K2_GetComponentRotation` _staticmeshcomponent) true true (`KismetMathLibrary.Conv_IntToDouble` (* (`KismetMathLibrary.Abs_Int` (- (`self.NewFloor`) (`self.CurrentFloor`))) 6)) :!label _label_4)
            (`self.ElevatorDeactivate`)
            (set `self.Activate` false)
            (set `self.IsFloorButton` false)
            (`PrimitiveComponent.SetMaterial` (cast `StaticMeshComponent` (`|GetArrayItem` (`self.FloorsArray`) (`self.IndexFloor`)) :!pure true) 1 "/Game/Assets/Geometry/Elevator/BaseEmissive_Inst.BaseEmissive_Inst")
            (if (not (`self.StopButton`))
              (`self.OpenDoors_Event`)
              (add `self.CloseDoors` (delegate `CustomEvent`) :!label _label_5)
              (else
                (`KismetSystemLibrary.Delay` 3.0 :!label _label_6)
                (if (not (`self.Activate`))
                  (`self.ElevatorDeactivateOnDowntime`)
                  (set `self.IsCall` false)
                  (set `self.StopButton` false)
                  (`PrimitiveComponent.SetMaterial` (`self.stop`) 1 "/Game/Assets/Geometry/Elevator/BaseEmissive_Inst.BaseEmissive_Inst"))))
            (elif (`self.IsEqualityHeight`)
              (`self.OpenDoors_Event`)
              (goto _label_5)
              (else
                (set `self.Activate` true :!label _label_7)
                (`PrimitiveComponent.SetMaterial` (`self.stop`) 1 "/Game/Assets/Geometry/Elevator/BaseEmissive_Inst.BaseEmissive_Inst")
                (`self.ElevatorActivate`)
                (`KismetSystemLibrary.MoveComponentTo` (`self.StaticMeshComponent`) (`KismetMathLibrary.MakeVector` (.x (`SceneComponent.K2_GetComponentLocation` (`self.StaticMeshComponent`))) (.y (`SceneComponent.K2_GetComponentLocation` (`self.StaticMeshComponent`))) _returnvalue) (`SceneComponent.K2_GetComponentRotation` (`self.StaticMeshComponent`)) true true (/ (`KismetMathLibrary.Abs` (- (.z (`SceneComponent.K2_GetComponentLocation` (`self.StaticMeshComponent`))) _returnvalue)) 20.0))
                (`self.ElevatorDeactivate`)
                (set `self.Activate` false)
                (set `self.IsFloorButton` false)
                (`PrimitiveComponent.SetMaterial` (cast `StaticMeshComponent` (`|GetArrayItem` (`self.FloorsArray`) (`self.IndexFloor`)) :!pure true) 1 "/Game/Assets/Geometry/Elevator/BaseEmissive_Inst.BaseEmissive_Inst")
                (`self.OpenDoors_Event`)
                (goto _label_5)))))))))

(event `UpDown`
  (params (Hit :type "HitResult Structure") (CallButton :type "/Game/Assets/Geometry/Elevator/BP_CallButton Object Reference"))
  (bind (_bblockinghit _binitialoverlap _time _distance _location _impactpoint _normal _impactnormal _physmat _hitactor _hitcomponent) (`GameplayStatics.BreakHitResult` Hit))
  (bind _stop (`self.stop`))
  (bind _returnvalue (`KismetArrayLibrary.Array_Find` (`self.FloorsArray`) _hitcomponent))
  ;[1 1 1] Main Logic
  (if (not (`self.Activate`))
    (`|ExecutionSequence`
      (:`then_0`
        (if (and (not (`self.IsCall`)) (not (`self.Activate`)) (== CallButton _hitactor))
          (`self.ButtonActivate`)
          (set `self.IsCall` true)
          (set `self.StopButton` false)
          (if (`self.OpenDoors`)
            (add `self.CloseDoors` (delegate `Event1`))
            (goto _label :!via `Reset`)
            (else
              (goto _label_2)))))
      (:`then_1`
        (if (== _hitcomponent _stop) :!label _label_8
          (set `self.StopButton` true)
          (`PrimitiveComponent.SetMaterial` _stop 1 "/Game/Assets/Geometry/Elevator/BaseEmissive_Inst1.BaseEmissive_Inst1")
          (`self.ElevatorDeactivate`)
          (set `self.IsCall` false)
          (set `self.IsFloorButton` false)
          (goto _label_4 :!via `Stop`)))
      (:`then_2`
        (if (and (>= _returnvalue 0) (not (`self.IsFloorButton`)))
          (bind _output_get (set `self.IndexFloor` _returnvalue))
          (set `self.IsFloorButton` true)
          (`PrimitiveComponent.SetMaterial` (cast `StaticMeshComponent` (`|GetArrayItem` (`self.FloorsArray`) _output_get) :!pure true) 1 "/Game/Assets/Geometry/Elevator/BaseEmissive_Inst1.BaseEmissive_Inst1")
          (set `self.StopButton` false)
          (if (`self.OpenDoors`)
            (add `self.CloseDoors` (delegate `Event2`))
            (goto _label_10 :!via `Reset`)
            (else
              (if (not (`self.Activate`)) :!label _label_9
                (bind _output_get_2 (set `self.NewFloor` (+ _output_get 1)))
                (if (!= _output_get_2 (`self.GetCurrentFloor`))
                  (`self.ButtonActivate`)
                  (goto _label_3)
                  (elif (`self.IsEqualityHeight`)
                    (`self.OpenDoors_Event`)
                    (`PrimitiveComponent.SetMaterial` (cast `StaticMeshComponent` (`|GetArrayItem` (`self.FloorsArray`) (`self.IndexFloor`)) :!pure true) 1 "/Game/Assets/Geometry/Elevator/BaseEmissive_Inst.BaseEmissive_Inst")
                    (set `self.IsFloorButton` false)
                    (else
                      (`self.ButtonActivate`)
                      (goto _label_7))))))))))
    (else
      (goto _label_8))))

(event `CustomEvent`
  ;[1 1 1] Main Logic
  (goto _label_6))

(event `Event2`
  ;[1 1 1] Main Logic
  (if (`self.StopButton`)
    (goto _label_4 :!via `Stop`)
    (else
      (`/Engine/EditorBlueprintResources/StandardMacros.DoOnce` false :!label _label_10
        (:`Completed`
          (goto _label_9))))))

(event `CloseDoors_Event`
  (bind _returnvalue_location (`KismetMathLibrary.BreakTransform` (`SceneComponent.GetRelativeTransform` (`self.R_Door`))))
  (bind _returnvalue_location_2 (`KismetMathLibrary.BreakTransform` (`SceneComponent.GetRelativeTransform` (`self.L_Door`))))
  ;[1 1 1] Close Doors
  (`/Game/Assets/Geometry/Elevator/BP_ElevatorDoors.CloseDoors` (`self.ActiveDoors`))
  (`AudioComponent.Play` (`self.elevator-door-open`) 0.0)
  (`|ExecutionSequence`
    (:`then_0`
      (`KismetSystemLibrary.MoveComponentTo` (`self.L_Door`) (`KismetMathLibrary.MakeVector` (.x _returnvalue_location_2) (- (.y _returnvalue_location_2) 63.0) (.z _returnvalue_location_2)) (struct) true true 3.0))
    (:`then_1`
      (`KismetSystemLibrary.MoveComponentTo` (`self.R_Door`) (`KismetMathLibrary.MakeVector` (.x _returnvalue_location) (+ (.y _returnvalue_location) 63.0) (.z _returnvalue_location)) (struct) true true 3.0)))
  (set `self.OpenDoors` false)
  (`self.CloseDoors`))

(event `OpenDoors_Event`
  (bind _returnvalue_location (`KismetMathLibrary.BreakTransform` (`SceneComponent.GetRelativeTransform` (`self.L_Door`))))
  (bind _returnvalue_location_2 (`KismetMathLibrary.BreakTransform` (`SceneComponent.GetRelativeTransform` (`self.R_Door`))))
  (bind _asbp_elevator_doors (cast `/Game/Assets/Geometry/Elevator/BP_ElevatorDoors` (`|GetArrayItem` (`PrimitiveComponent.GetOverlappingActors` (`self.RegisterDoorFloor`) "/Game/Assets/Geometry/Elevator/BP_ElevatorDoors.BP_ElevatorDoors_C")) :!pure true))
  ;[1 1 1] Open Doors
  (`KismetSystemLibrary.Delay` 0.2)
  (`/Game/Assets/Geometry/Elevator/BP_ElevatorDoors.OpenDoors` _asbp_elevator_doors 0)
  (set `self.ActiveDoors` _asbp_elevator_doors)
  (`AudioComponent.Play` (`self.elevator-door-open`) 0.0)
  (`PrimitiveComponent.SetMaterial` (`self.stop`) 1 "/Game/Assets/Geometry/Elevator/BaseEmissive_Inst.BaseEmissive_Inst")
  (set `self.OpenDoors` true)
  (`|ExecutionSequence`
    (:`then_1`
      (`|ExecutionSequence`
        (:`then_0`
          (`KismetSystemLibrary.MoveComponentTo` (`self.L_Door`) (`KismetMathLibrary.MakeVector` (.x _returnvalue_location) (+ (.y _returnvalue_location) 63.0) (.z _returnvalue_location)) (struct) true true 3.0))
        (:`then_1`
          (`KismetSystemLibrary.MoveComponentTo` (`self.R_Door`) (`KismetMathLibrary.MakeVector` (.x _returnvalue_location_2) (- (.y _returnvalue_location_2) 63.0) (.z _returnvalue_location_2)) (struct) true true 3.0)))
      (`KismetSystemLibrary.Delay` 4.0)
      (`self.CloseDoors_Event`))))

(fn `GetCurrentFloor`
  (returns (CurrentFloor :type Integer))
  (bind _output_get (set `self.CurrentFloor` (+ (`KismetMathLibrary.Round` (/ (- (+ (.z (`SceneComponent.K2_GetComponentLocation` (`self.StaticMeshComponent`))) 20.0) (`self.GetHeightFirstFloor` (`self.Building`))) (`KismetMathLibrary.Conv_IntToDouble` (`self.HeightFloor`)))) 1)))
  (return _output_get))

(fn `GetHeightFirstFloor`
  (params (Building :type "StaticMeshActor Object Reference"))
  (returns (HeightFirstFloor :type "Float (double-precision)"))
  (bind _output_get (set `self.HeightFirstFloor` (+ (.z (`SceneComponent.K2_GetComponentLocation` (`Actor.RootComponent` Building))) 200.0)))
  (return _output_get))

(fn `Interact`
  (params (Character :type "/Game/Blueprints/Characters/BP_PlayerCharacter Object Reference") (Hit :type "HitResult Structure"))
  (returns (Success :type Boolean))
  (`self.UpDown` Hit)
  (return true))

(fn `IsEqualityHeight`
  (returns (Equal :type Boolean))
  (return (== (`KismetMathLibrary.Round` (.z (`SceneComponent.K2_GetComponentLocation` (`self.StaticMeshComponent`)))) (`KismetMathLibrary.Round` (+ (`self.HeightFirstFloor`) (`KismetMathLibrary.Conv_IntToDouble` (- (* (- (`self.CurrentFloor`) 1) (`self.HeightFloor`)) 20)))))))

(fn `UserConstructionScript`
  (bind _output_get (set `self.FloorsArray` (`SceneComponent.GetChildrenComponents` (`self.command bar`) true)))
  (set `self.NumberOfFloors` (`KismetArrayLibrary.Array_Length` _output_get)))