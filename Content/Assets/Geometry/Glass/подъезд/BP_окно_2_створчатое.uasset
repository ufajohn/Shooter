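; Breakable two-sash apartment-entrance window whose glass shatters when another actor begins overlapping it.
; The overlap applies small radius damage to the destructible component at that actor's location and plays a lower-pitched breaking sound at the window mesh.
; The construction script loops over every instance of this window class, not just itself, zeroing the large-chunk threshold and randomly assigning one of five glass materials.
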(event `self.DestructibleComponent0.OnComponentBeginOverlap`
  (params (OverlappedComponent :type "PrimitiveComponent Object Reference") (OtherActor :type "Actor Object Reference") (OtherComp :type "PrimitiveComponent Object Reference") (OtherBodyIndex :type Integer) (bFromSweep :type Boolean) (SweepResult :type "HitResult Structure (by ref)"))
  (`DestructibleComponent.ApplyRadiusDamage` (`self.DestructibleComponent0`) 10.0 (`self.K2_GetActorLocation` OtherActor) 30.0 1.0 false)
  (`GameplayStatics.SpawnSoundAtLocation` "/Game/Assets/Geometry/Glass/BreakGlass_Cue.BreakGlass_Cue" (`SceneComponent.K2_GetComponentLocation` (`self.окно_3_створчатое_Mesh1`)) (struct) 1.0 0.8 0.0 "/Game/Assets/Geometry/Glass/GlassSoundAttenuation.GlassSoundAttenuation" null))

(fn `UserConstructionScript`
  (bind (_glass1 _glass2 _glass3 _glass4 _glass5) (break `/Game/AdvancedGlassPack/Materials/04_Shattered/_Examples/GlassStructure` (`self.GlassStructure`)))
  (bind _outactors (`GameplayStatics.GetAllActorsOfClass` "BP_окно_2_створчатое_C"))
  (for _array_element _outactors
    (bind _destructiblecomponent0 (`/Game/Assets/Geometry/Glass/подъезд/BP_окно_2_створчатое.DestructibleComponent0` _array_element))
    (set `DestructibleComponent.LargeChunkThreshold` 0.0 _destructiblecomponent0)
    (`PrimitiveComponent.SetMaterial` _destructiblecomponent0 0 (select `int` (`KismetMathLibrary.RandomIntegerInRange` 0 4) :`0` _glass1 :`1` _glass2 :`2` _glass3 :`3` _glass4 :`4` _glass5))))