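; Breakable glass balcony door Blueprint built on a destructible component.
; When another actor begins overlapping it, the component takes small radius damage centered on that actor's location.
; Its construction script loops over every BP_балконная_дверь actor, a class name without this file's "1" suffix, assigning each a random glass material from five variants.
; A glass-breaking sound spawn exists but is unconnected and never runs.
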(event `self.DestructibleComponent0.OnComponentBeginOverlap`
  (params (OverlappedComponent :type "PrimitiveComponent Object Reference") (OtherActor :type "Actor Object Reference") (OtherComp :type "PrimitiveComponent Object Reference") (OtherBodyIndex :type Integer) (bFromSweep :type Boolean) (SweepResult :type "HitResult Structure (by ref)"))
  (`DestructibleComponent.ApplyRadiusDamage` (`self.DestructibleComponent0`) 10.0 (`self.K2_GetActorLocation` OtherActor) 30.0 1.0 false))

(fn `UserConstructionScript`
  (bind (_glass1 _glass2 _glass3 _glass4 _glass5) (break `/Game/AdvancedGlassPack/Materials/04_Shattered/_Examples/GlassStructure` (`self.GlassStructure`)))
  (bind _outactors (`GameplayStatics.GetAllActorsOfClass` "/Game/Assets/Geometry/Glass/балконная_дверь/BP_балконная_дверь.BP_балконная_дверь_C"))
  (for _array_element _outactors
    (`PrimitiveComponent.SetMaterial` (`/Game/Assets/Geometry/Glass/балконная_дверь/BP_балконная_дверь.DestructibleComponent0` _array_element) 0 (select `int` (`KismetMathLibrary.RandomIntegerInRange` 0 4) :`0` _glass1 :`1` _glass2 :`2` _glass3 :`3` _glass4 :`4` _glass5))))