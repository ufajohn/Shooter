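; Breakable stained-glass window built from destructible glass panes.
; Overlapping any of ten panes applies small radius damage to it at the other actor's location and plays a shared breaking sound at the window mesh.
; The construction script loops over every instance of this class, not just itself, setting chunk thresholds and random materials on Up and Down child panes from separate glass structs.
; The Down selection repeats Glass2 and never uses Glass3.
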(event `self.плейс_лит1_Mesh1_DM.OnComponentBeginOverlap`
  (params (OverlappedComponent :type "PrimitiveComponent Object Reference") (OtherActor :type "Actor Object Reference") (OtherComp :type "PrimitiveComponent Object Reference") (OtherBodyIndex :type Integer) (bFromSweep :type Boolean) (SweepResult :type "HitResult Structure (by ref)"))
  (`DestructibleComponent.ApplyRadiusDamage` (`self.плейс_лит1_Mesh1_DM`) 10.0 (`self.K2_GetActorLocation` OtherActor) 20.0 1.0 false)
  (`GameplayStatics.SpawnSoundAtLocation` "/Game/Assets/Geometry/Glass/BreakGlass_Cue.BreakGlass_Cue" (`SceneComponent.K2_GetComponentLocation` (`self.окно_3_створчатое_Mesh1`)) (struct) 1.0 0.8 0.0 "/Game/Assets/Geometry/Glass/GlassSoundAttenuation.GlassSoundAttenuation" null :!label _label))

(event `self.плейс_лит1_Mesh2_DM.OnComponentBeginOverlap`
  (params (OverlappedComponent :type "PrimitiveComponent Object Reference") (OtherActor :type "Actor Object Reference") (OtherComp :type "PrimitiveComponent Object Reference") (OtherBodyIndex :type Integer) (bFromSweep :type Boolean) (SweepResult :type "HitResult Structure (by ref)"))
  (`DestructibleComponent.ApplyRadiusDamage` (`self.плейс_лит1_Mesh2_DM`) 10.0 (`self.K2_GetActorLocation` OtherActor) 20.0 1.0 false)
  (goto _label))

(event `self.плейс_лит1_Mesh3_DM.OnComponentBeginOverlap`
  (params (OverlappedComponent :type "PrimitiveComponent Object Reference") (OtherActor :type "Actor Object Reference") (OtherComp :type "PrimitiveComponent Object Reference") (OtherBodyIndex :type Integer) (bFromSweep :type Boolean) (SweepResult :type "HitResult Structure (by ref)"))
  (`DestructibleComponent.ApplyRadiusDamage` (`self.плейс_лит1_Mesh3_DM`) 10.0 (`self.K2_GetActorLocation` OtherActor) 20.0 1.0 false)
  (goto _label))

(event `self.плейс_лит1_Mesh4_DM.OnComponentBeginOverlap`
  (params (OverlappedComponent :type "PrimitiveComponent Object Reference") (OtherActor :type "Actor Object Reference") (OtherComp :type "PrimitiveComponent Object Reference") (OtherBodyIndex :type Integer) (bFromSweep :type Boolean) (SweepResult :type "HitResult Structure (by ref)"))
  (`DestructibleComponent.ApplyRadiusDamage` (`self.плейс_лит1_Mesh4_DM`) 10.0 (`self.K2_GetActorLocation` OtherActor) 20.0 1.0 false)
  (goto _label))

(event `self.плейс_лит1_Mesh5_DM.OnComponentBeginOverlap`
  (params (OverlappedComponent :type "PrimitiveComponent Object Reference") (OtherActor :type "Actor Object Reference") (OtherComp :type "PrimitiveComponent Object Reference") (OtherBodyIndex :type Integer) (bFromSweep :type Boolean) (SweepResult :type "HitResult Structure (by ref)"))
  (`DestructibleComponent.ApplyRadiusDamage` (`self.плейс_лит1_Mesh5_DM`) 10.0 (`self.K2_GetActorLocation` OtherActor) 20.0 1.0 false)
  (goto _label))

(event `self.плейс_лит1_Mesh6_DM.OnComponentBeginOverlap`
  (params (OverlappedComponent :type "PrimitiveComponent Object Reference") (OtherActor :type "Actor Object Reference") (OtherComp :type "PrimitiveComponent Object Reference") (OtherBodyIndex :type Integer) (bFromSweep :type Boolean) (SweepResult :type "HitResult Structure (by ref)"))
  (`DestructibleComponent.ApplyRadiusDamage` (`self.плейс_лит1_Mesh6_DM`) 10.0 (`self.K2_GetActorLocation` OtherActor) 20.0 1.0 false)
  (goto _label))

(event `self.плейс_лит1_Mesh7_DM.OnComponentBeginOverlap`
  (params (OverlappedComponent :type "PrimitiveComponent Object Reference") (OtherActor :type "Actor Object Reference") (OtherComp :type "PrimitiveComponent Object Reference") (OtherBodyIndex :type Integer) (bFromSweep :type Boolean) (SweepResult :type "HitResult Structure (by ref)"))
  (`DestructibleComponent.ApplyRadiusDamage` (`self.плейс_лит1_Mesh7_DM`) 10.0 (`self.K2_GetActorLocation` OtherActor) 20.0 1.0 false)
  (goto _label))

(event `self.плейс_лит1_Mesh8_DM.OnComponentBeginOverlap`
  (params (OverlappedComponent :type "PrimitiveComponent Object Reference") (OtherActor :type "Actor Object Reference") (OtherComp :type "PrimitiveComponent Object Reference") (OtherBodyIndex :type Integer) (bFromSweep :type Boolean) (SweepResult :type "HitResult Structure (by ref)"))
  (`DestructibleComponent.ApplyRadiusDamage` (`self.плейс_лит1_Mesh8_DM`) 10.0 (`self.K2_GetActorLocation` OtherActor) 20.0 1.0 false)
  (goto _label))

(event `self.плейс_лит1_Mesh9_DM.OnComponentBeginOverlap`
  (params (OverlappedComponent :type "PrimitiveComponent Object Reference") (OtherActor :type "Actor Object Reference") (OtherComp :type "PrimitiveComponent Object Reference") (OtherBodyIndex :type Integer) (bFromSweep :type Boolean) (SweepResult :type "HitResult Structure (by ref)"))
  (`DestructibleComponent.ApplyRadiusDamage` (`self.плейс_лит1_Mesh9_DM`) 10.0 (`self.K2_GetActorLocation` OtherActor) 20.0 1.0 false)
  (goto _label))

(event `self.плейс_лит1_Mesh10_DM.OnComponentBeginOverlap`
  (params (OverlappedComponent :type "PrimitiveComponent Object Reference") (OtherActor :type "Actor Object Reference") (OtherComp :type "PrimitiveComponent Object Reference") (OtherBodyIndex :type Integer) (bFromSweep :type Boolean) (SweepResult :type "HitResult Structure (by ref)"))
  (`DestructibleComponent.ApplyRadiusDamage` (`self.плейс_лит1_Mesh10_DM`) 10.0 (`self.K2_GetActorLocation` OtherActor) 20.0 1.0 false)
  (goto _label))

(fn `UserConstructionScript`
  (bind (_glass1 _glass2 _glass3 _glass4 _glass5) (break `/Game/AdvancedGlassPack/Materials/04_Shattered/_Examples/GlassStructure` (`self.GlassStructure`)))
  (bind (_glass1_2 _glass2_2 _glass3_2 _glass4_2 _glass5_2) (break `/Game/AdvancedGlassPack/Materials/04_Shattered/_Examples/GlassStructure2` (`self.GlassStructure2`)))
  (bind _outactors (`GameplayStatics.GetAllActorsOfClass` "BP_витраж3355_C"))
  (for _array_element _outactors
    (`|ExecutionSequence`
      (:`then_0`
        (for _array_element_2 (`SceneComponent.GetChildrenComponents` (`/Game/Assets/Geometry/Glass/витраж3355/BP_витраж3355.Up` _array_element) false)
          (bind _asdestructible_component (cast `DestructibleComponent` _array_element_2 :!pure true))
          (set `DestructibleComponent.LargeChunkThreshold` 50.0 _asdestructible_component)
          (`PrimitiveComponent.SetMaterial` _asdestructible_component 0 (select `int` (`KismetMathLibrary.RandomIntegerInRange` 0 4) :`0` _glass1 :`1` _glass2 :`2` _glass3 :`3` _glass4 :`4` _glass5))))
      (:`then_1`
        (for _array_element_3 (`SceneComponent.GetChildrenComponents` (`/Game/Assets/Geometry/Glass/витраж3355/BP_витраж3355.Down` _array_element) false)
          (bind _asdestructible_component_2 (cast `DestructibleComponent` _array_element_3 :!pure true))
          (set `DestructibleComponent.LargeChunkThreshold` 50.0 _asdestructible_component_2)
          (`PrimitiveComponent.SetMaterial` _asdestructible_component_2 0 (select `int` (`KismetMathLibrary.RandomIntegerInRange` 0 4) :`0` _glass1_2 :`1` _glass2_2 :`2` _glass2_2 :`3` _glass4_2 :`4` _glass5_2)))))))