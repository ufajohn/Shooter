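; Player state for the lobby that holds a player's info struct (name, image, pawn, pawn image, status, team ID) and handles status changes.
; SetPlayerStatus changes only the status member and passes the struct to SendToServer.
; SendToServer stores the struct, then casts the game state to LobbyGameState and calls UpdatePlayerList to refresh the player list.
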(event `SetPlayerStatus`
  (params (MyPlayerStatus :type Text))
  (bind _playerinfo_0 (`self.PlayerInfo_0`))
  (bind (_myplayername _myplayerimage _myplayerpawn _myplayerpawnimage _myplayerstatus _myplayerteamid) (break `/Game/Blueprints/General/PlayerInfo` _playerinfo_0))
  ;[1 1 1] Set Player Status
  (bind _structout (setmembers `/Game/Blueprints/General/PlayerInfo` :`StructRef` _playerinfo_0 :`MyPlayerName` _myplayername :`MyPlayerImage` _myplayerimage :`MyPlayerPawn` _myplayerpawn :`MyPlayerPawnImage` _myplayerpawnimage :`MyPlayerStatus` MyPlayerStatus :`MyPlayerTeamID` _myplayerteamid))
  (`self.SendToServer` _structout))

(event `SendToServer`
  (params (PlayerInfo :type "/Game/Blueprints/General/PlayerInfo Structure"))
  ;[1 1 1] Send Status to Server
  (set `self.PlayerInfo_0` PlayerInfo)
  (bind _aslobby_game_state (cast `/Game/Blueprints/Lobby/LobbyGameState` (`GameplayStatics.GetGameState`)))
  (`/Game/Blueprints/Lobby/LobbyGameState.UpdatePlayerList` _aslobby_game_state))

(fn `UserConstructionScript`
  (`parent.UserConstructionScript`))