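; Lobby game mode that keeps the lobby's player list in step as players join, swap controllers or leave.
; PostLogin adds the player to LobbyGameState, runs InitialSetup on its LobbyPlayerController, then refreshes the list.
; Controller swaps re-add and refresh without repeating setup, while logout removes the player and refreshes the list twice.
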(event `self.K2_PostLogin`
  (params (NewPlayer :type "PlayerController Object Reference"))
  ;[1 1 1] Handle Login and Logout
  (bind _aslobby_game_state (cast `/Game/Blueprints/Lobby/LobbyGameState` (`GameplayStatics.GetGameState`)))
  (`/Game/Blueprints/Lobby/LobbyGameState.AddPlayer` _aslobby_game_state NewPlayer)
  (bind _aslobby_player_controller (cast `/Game/Blueprints/Lobby/LobbyPlayerController` NewPlayer))
  (`/Game/Blueprints/Lobby/LobbyPlayerController.InitialSetup` _aslobby_player_controller)
  (`/Game/Blueprints/Lobby/LobbyGameState.UpdatePlayerList` _aslobby_game_state))

(event `self.K2_OnSwapPlayerControllers`
  (params (OldPC :type "PlayerController Object Reference") (NewPC :type "PlayerController Object Reference"))
  ;[1 1 1] Handle Login and Logout
  (bind _aslobby_game_state (cast `/Game/Blueprints/Lobby/LobbyGameState` (`GameplayStatics.GetGameState`)))
  (`/Game/Blueprints/Lobby/LobbyGameState.AddPlayer` _aslobby_game_state NewPC)
  (cast `/Game/Blueprints/Lobby/LobbyPlayerController` NewPC)
  (`/Game/Blueprints/Lobby/LobbyGameState.UpdatePlayerList` _aslobby_game_state))

(event `self.K2_OnLogout`
  (params (ExitingController :type "Controller Object Reference"))
  ;[1 1 1] Handle Login and Logout
  (bind _aslobby_game_state (cast `/Game/Blueprints/Lobby/LobbyGameState` (`GameplayStatics.GetGameState`)))
  (`/Game/Blueprints/Lobby/LobbyGameState.RemovePlayer` _aslobby_game_state null)
  (`/Game/Blueprints/Lobby/LobbyGameState.UpdatePlayerList` _aslobby_game_state)
  (`/Game/Blueprints/Lobby/LobbyGameState.UpdatePlayerList` _aslobby_game_state))

(fn `UserConstructionScript`)