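; Blueprint function library of global getters for the game's core framework objects.
; Each function fetches the current game state, game instance, game mode or player controller and casts it to the project's class, returning nothing useful if the cast fails.
; Base and derived variants exist for game mode and game state, and the player controller getter always uses player index 0.
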(fn `GetBP_BaseGameMode`
  (returns (`AsBP Base Game Mode` :type "/Game/Blueprints/Gameplay/BP_BaseGameMode Object Reference"))
  (bind _asbp_base_game_mode (cast `/Game/Blueprints/Gameplay/BP_BaseGameMode` (`GameplayStatics.GetGameMode` null)))
  (return _asbp_base_game_mode))

(fn `GetBP_BaseGameState`
  (returns (`AsBP Game State Base` :type "/Game/Blueprints/Gameplay/BP_GameStateBase Object Reference"))
  (bind _asbp_game_state_base (cast `/Game/Blueprints/Gameplay/BP_GameStateBase` (`GameplayStatics.GetGameState` null)))
  (return _asbp_game_state_base))

(fn `GetBP_GameMode`
  (returns (`AsBP Game Mode` :type "/Game/Blueprints/Gameplay/BP_GameMode Object Reference"))
  (bind _asbp_game_mode (cast `/Game/Blueprints/Gameplay/BP_GameMode` (`GameplayStatics.GetGameMode` null)))
  (return _asbp_game_mode))

(fn `GetBP_GameState`
  (returns (`AsBP Game State` :type "/Game/Blueprints/Gameplay/BP_GameState Object Reference"))
  (bind _asbp_game_state (cast `/Game/Blueprints/Gameplay/BP_GameState` (`GameplayStatics.GetGameState` null)))
  (return _asbp_game_state))

(fn `GetBP_PlayerController`
  (returns (`AsBP Player Controller` :type "/Game/Blueprints/Characters/BP_PlayerController Object Reference"))
  (bind _asbp_player_controller (cast `/Game/Blueprints/Characters/BP_PlayerController` (`GameplayStatics.GetPlayerController` null)))
  (return _asbp_player_controller))

(fn `GetGlobalGameInstance`
  (returns (`AsGlobal Game Instance` :type "/Game/Blueprints/General/GlobalGameInstance Object Reference"))
  (bind _asglobal_game_instance (cast `/Game/Blueprints/General/GlobalGameInstance` (`GameplayStatics.GetGameInstance` null)))
  (return _asglobal_game_instance))