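; Health component for BP_PlayerCharacter that tracks health and armor and reports deaths to BP_GameMode.
; Initializes both values to maximums and binds the owner's any-damage event on the server only.
; Armor divides damage by a tenth of its value, then drops by raw damage; without armor, health takes full damage.
; Death is reported on lethal unarmored hits or any hit at depleted health, not on the armored hit that depletes it.
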(event `self.ReceiveBeginPlay`
  (set `self.health` (`self.maxHealth`))
  (set `self.armor` (`self.maxArmor`))
  (bind _asbp_player_character (cast `/Game/Blueprints/Characters/BP_PlayerCharacter` (`self.GetOwner`)))
  (bind _output_get (set `self.DamageCharacter` _asbp_player_character))
  (if (`KismetSystemLibrary.IsServer`)
    (add `Actor.OnTakeAnyDamage` _output_get (delegate `OnTakeAnyDamage_Event_0`))))

(event `OnTakeAnyDamage_Event_0`
  (params (DamagedActor :type "Actor Object Reference") (Damage :type "Float (double-precision)") (DamageType :type "DamageType Object Reference") (InstigatedBy :type "Controller Object Reference") (DamageCauser :type "Actor Object Reference"))
  (if (and (> (`self.health`) 0.0) (> (`self.armor`) 0.0))
    (set `self.health` (- (`self.health`) (/ Damage (* (`self.armor`) 0.1))))
    (set `self.armor` (`KismetMathLibrary.FMax` (- (`self.armor`) Damage)))
    (elif (and (> (`self.health`) 0.0) (<= (`self.armor`) 0.0))
      (bind _output_get (set `self.health` (`KismetMathLibrary.FMax` (- (`self.health`) Damage))))
      (if (<= _output_get 0.0)
        (if (`KismetSystemLibrary.IsValid` (`Pawn.PlayerState` (`self.DamageCharacter`))) :!label _label
          (`/Game/Blueprints/Gameplay/BP_GameMode.CharacterDeath` (cast `/Game/Blueprints/Gameplay/BP_GameMode` (`GameplayStatics.GetGameMode`) :!pure true) (`self.DamageCharacter`) (cast `/Game/Blueprints/Characters/BP_PlayerController` InstigatedBy :!pure true) DamageCauser)))
      (else
        (goto _label)))))