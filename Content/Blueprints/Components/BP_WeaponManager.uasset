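; Weapon manager component for BP_PlayerCharacter that holds main, secondary and melee weapons and handles equipping, switching and dropping them.
; Add, select and scroll events update InventoryStructure and CurrentWeapon, toggling actor visibility through OnServer events that call All events.
; Dropping places the weapon before the owner, clears its slot and auto-selects the first remaining one.
; Separate array-based functions, including Special and Grenade types, are partly stubbed or disconnected.
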(event `self.ReceiveBeginPlay`
  ;[1 1 1] Get Owner Character
  (set `self.OwnerWeaponManager` (cast `/Game/Blueprints/Characters/BP_PlayerCharacter` (`self.GetOwner`) :!pure true)))

(event `self.ReceiveTick`
  (params (DeltaSeconds :type "Float (single-precision)")))

(event `AddWeaponInInventoryOnServer`
  (params (Owner :type "/Game/Blueprints/Characters/BP_PlayerCharacter Object Reference") (NewWeapon :type "/Game/Blueprints/Weapons/BP_Weapon Object Reference"))
  (bind (_asbp_weapon_auto_rifles _bsuccess) (cast `/Game/Blueprints/Weapons/BP_Weapon_AutoRifles` NewWeapon :!pure true))
  (bind (_asbp_weapon_pistols _bsuccess_2) (cast `/Game/Blueprints/Weapons/BP_Weapon_Pistols` NewWeapon :!pure true))
  (bind (_asbp_weapon_knife _bsuccess_3) (cast `/Game/Blueprints/Weapons/BP_Weapon_Knife` NewWeapon :!pure true))
  ;[1 1 1] Add Weapon in the Inventory
  (set `/Game/Blueprints/Weapons/BP_Weapon.WeaponOwner` Owner NewWeapon)
  (bind _currentweapon (`self.CurrentWeapon`)
    (:`then`
      (`Actor.SetActorHiddenInGame` _currentweapon true))
    (:`else`
      _))
  (switch `/Game/Data/E_WeaponType` (`/Game/Blueprints/Weapons/BP_Weapon.weaponType` NewWeapon)
    (:`NewEnumerator0`
      (if _bsuccess
        (setmembers `/Game/Blueprints/Weapons/BP_WeaponInventory` :`StructRef` (`self.InventoryStructure`) :`MainWeapon` _asbp_weapon_auto_rifles)
        (set `self.CurrentWeapon` _asbp_weapon_auto_rifles)
        (set `self.MainWeapon` _asbp_weapon_auto_rifles)
        (`Actor.SetActorHiddenInGame` _asbp_weapon_auto_rifles false)))
    (:`NewEnumerator1`
      (if _bsuccess_2
        (setmembers `/Game/Blueprints/Weapons/BP_WeaponInventory` :`StructRef` (`self.InventoryStructure`) :`SecondWeapon` _asbp_weapon_pistols)
        (set `self.CurrentWeapon` _asbp_weapon_pistols)
        (set `self.SecondWeapon` _asbp_weapon_pistols)
        (`Actor.SetActorHiddenInGame` _asbp_weapon_pistols false)))
    (:`NewEnumerator4`
      (if _bsuccess_3
        (setmembers `/Game/Blueprints/Weapons/BP_WeaponInventory` :`StructRef` (`self.InventoryStructure`) :`MeleeWeapon` _asbp_weapon_knife)
        (set `self.CurrentWeapon` _asbp_weapon_knife)
        (set `self.MeleeWeapon` _asbp_weapon_knife)
        (`Actor.SetActorHiddenInGame` _asbp_weapon_knife false)))))

(event `SelectWeaponOnClient`
  (params (Type :type "/Game/Data/E_WeaponType Enum" :default "NewEnumerator0"))
  (bind (_mainweapon _secondweapon _meleeweapon) (break `/Game/Blueprints/Weapons/BP_WeaponInventory` (`self.InventoryStructure`)))
  ;[1 1 1] Select Weapon and Set
  (`|ExecutionSequence`
    (:`then_0`
      (if (`|EnumEquality` Type "NewEnumerator0")
        (`/Engine/EditorBlueprintResources/StandardMacros.IsValid` _mainweapon
          (:`Is Valid`
            (bind _currentweapon (`self.CurrentWeapon`)
              (:`then`
                (`self.HiddenWeaponOnServer` _currentweapon))
              (:`else`
                _))
            (bind _output_get (set `self.CurrentWeapon` _mainweapon))
            (`self.ShowCurrentWeaponOnServer` _output_get)))))
    (:`then_1`
      (if (`|EnumEquality` Type "NewEnumerator1")
        (`/Engine/EditorBlueprintResources/StandardMacros.IsValid` _secondweapon
          (:`Is Valid`
            (bind _currentweapon_2 (`self.CurrentWeapon`)
              (:`then`
                (`self.HiddenWeaponOnServer` _currentweapon_2))
              (:`else`
                _))
            (bind _output_get_2 (set `self.CurrentWeapon` _secondweapon))
            (`self.ShowCurrentWeaponOnServer` _output_get_2)))))
    (:`then_2`
      (if (`|EnumEquality` Type "NewEnumerator4")
        (`/Engine/EditorBlueprintResources/StandardMacros.IsValid` _meleeweapon
          (:`Is Valid`
            (bind _currentweapon_3 (`self.CurrentWeapon`)
              (:`then`
                (`self.HiddenWeaponOnServer` _currentweapon_3))
              (:`else`
                _))
            (bind _output_get_3 (set `self.CurrentWeapon` _meleeweapon))
            (`self.ShowCurrentWeaponOnServer` _output_get_3)))))))

(event `HiddenWeaponOnServer`
  (params (Weapon :type "/Game/Blueprints/Weapons/BP_Weapon Object Reference"))
  ;[1 1 1] Hidden Weapon
  (`self.HiddenWeaponAll` Weapon))

(event `ShowCurrentWeaponOnServer`
  (params (Weapon :type "/Game/Blueprints/Weapons/BP_Weapon Object Reference"))
  ;[1 1 1] Show Current Weapon
  (`self.ShowCurrentWeaponAll` Weapon))

(event `HiddenWeaponAll`
  (params (Weapon :type "/Game/Blueprints/Weapons/BP_Weapon Object Reference"))
  ;[1 1 1] Hidden Weapon
  (`Actor.SetActorHiddenInGame` Weapon true))

(event `ShowCurrentWeaponAll`
  (params (Weapon :type "/Game/Blueprints/Weapons/BP_Weapon Object Reference"))
  ;[1 1 1] Show Current Weapon
  (bind _output_get (set `self.CurrentWeapon` Weapon))
  (`Actor.SetActorHiddenInGame` _output_get false))

(event `ScrollWeaponEvent`
  (params (Up :type Boolean :default true))
  (bind (_mainweapon _secondweapon _meleeweapon) (break `/Game/Blueprints/Weapons/BP_WeaponInventory` (`self.InventoryStructure`)))
  (bind _weapontype (`/Game/Blueprints/Weapons/BP_Weapon.weaponType` (`self.CurrentWeapon`)))
  (bind _weapontype_2 (`/Game/Blueprints/Weapons/BP_Weapon.weaponType` (`self.CurrentWeapon`)))
  ;[1 1 1] ScrollWeapon
  (if Up
    (`|ExecutionSequence`
      (:`then_0`
        (if (`|EnumEquality` _weapontype_2 "NewEnumerator1")
          (`/Engine/EditorBlueprintResources/StandardMacros.IsValid` _mainweapon
            (:`Is Valid`
              (`self.HiddenWeaponOnServer` (`self.CurrentWeapon`))
              (bind _output_get (set `self.CurrentWeapon` _mainweapon))
              (`self.ShowCurrentWeaponOnServer` _output_get)))))
      (:`then_1`
        (if (`|EnumEquality` _weapontype_2 "NewEnumerator4")
          (`/Engine/EditorBlueprintResources/StandardMacros.IsValid` _secondweapon
            (:`Is Valid`
              (`self.HiddenWeaponOnServer` (`self.CurrentWeapon`))
              (bind _output_get_2 (set `self.CurrentWeapon` _secondweapon))
              (`self.ShowCurrentWeaponOnServer` _output_get_2))))))
    (else
      (`|ExecutionSequence`
        (:`then_0`
          (if (`|EnumEquality` _weapontype "NewEnumerator1")
            (`/Engine/EditorBlueprintResources/StandardMacros.IsValid` _meleeweapon
              (:`Is Valid`
                (`self.HiddenWeaponOnServer` (`self.CurrentWeapon`))
                (bind _output_get_3 (set `self.CurrentWeapon` _meleeweapon))
                (`self.ShowCurrentWeaponOnServer` _output_get_3)))))
        (:`then_1`
          (if (`|EnumEquality` _weapontype "NewEnumerator0")
            (`/Engine/EditorBlueprintResources/StandardMacros.IsValid` _secondweapon
              (:`Is Valid`
                (`self.HiddenWeaponOnServer` (`self.CurrentWeapon`))
                (bind _output_get_4 (set `self.CurrentWeapon` _secondweapon))
                (`self.ShowCurrentWeaponOnServer` _output_get_4)))))))))

(event `DropWeaponOnServer`
  (params (DroppedWeapon :type "/Game/Blueprints/Weapons/BP_Weapon Object Reference"))
  (bind _currentweapon (`self.CurrentWeapon`))
  ;[1 1 1] DropWeapon
  (`self.DropWeaponOnClients` DroppedWeapon)
  (set `/Game/Blueprints/Weapons/BP_Weapon.WeaponOwner` null _currentweapon)
  (switch `/Game/Data/E_WeaponType` (`/Game/Blueprints/Weapons/BP_Weapon.weaponType` _currentweapon)
    (:`NewEnumerator0`
      (set `self.MainWeapon` null))
    (:`NewEnumerator1`
      (set `self.SecondWeapon` null))
    (:`NewEnumerator4`
      (set `self.MeleeWeapon` null)))
  (setmembers `/Game/Blueprints/Weapons/BP_WeaponInventory` :`StructRef` (`self.InventoryStructure`) :`MainWeapon` (`self.MainWeapon`) :`SecondWeapon` (`self.SecondWeapon`) :`MeleeWeapon` (`self.MeleeWeapon`))
  (set `self.CurrentWeapon` null)
  (`self.AutosetWeaponOnServer`))

(event `DropWeaponOnClients`
  (params (DroppedWeapon :type "/Game/Blueprints/Weapons/BP_Weapon Object Reference"))
  (bind _ownerweaponmanager (`self.OwnerWeaponManager`))
  ;[1 1 1] DropWeapon
  (`Actor.K2_SetActorLocationAndRotation` DroppedWeapon (+ (`Actor.K2_GetActorLocation` _ownerweaponmanager) (* (`Actor.GetActorForwardVector` _ownerweaponmanager) 50.0)) (`Actor.K2_GetActorRotation` _ownerweaponmanager) false false))

(event `AutosetWeaponOnServer`
  ;[1 1 1] Autoset Weapon
  (bind _output_get (set `self.WeaponArray` (`|MakeArray` (`self.MainWeapon`) (`self.SecondWeapon`) (`self.MeleeWeapon`) :!type "/Game/Blueprints/Weapons/BP_Weapon Object Reference")))
  (for _array_element _output_get
    (`/Engine/EditorBlueprintResources/StandardMacros.IsValid` _array_element
      (:`Is Valid`
        (`self.SelectWeaponOnClient` (`/Game/Blueprints/Weapons/BP_Weapon.weaponType` _array_element))
        (break)))))

(fn `AddWeapon`
  (params (Owner :type "/Game/Blueprints/Characters/BP_PlayerCharacter Object Reference") (Weapon :type "/Game/Blueprints/Weapons/BP_Weapon Object Reference"))
  (locals (L_Weapon :type "/Game/Blueprints/Weapons/BP_Weapon Object Reference") (L_DropWeapon :type "/Game/Blueprints/Weapons/BP_Weapon Object Reference") (L_WeaponIndex :type Integer :default 0)))

(fn `AddWeaponInventoryType`
  (params (AddWeapon :type "/Game/Blueprints/Weapons/BP_Weapon Object Reference"))
  (`KismetArrayLibrary.Array_Add` (`self.InventoryType`) (`/Game/Blueprints/Weapons/BP_Weapon.weaponType` AddWeapon)))

(fn `AutosetWeapon`
  (params (DropedWeapon :type "/Game/Blueprints/Weapons/BP_Weapon Object Reference")))

(fn `CleanWeaponVariable`
  (params (Weapon :type "/Game/Blueprints/Weapons/BP_Weapon Object Reference"))
  (switch `/Game/Data/E_WeaponType` (`/Game/Blueprints/Weapons/BP_Weapon.weaponType` Weapon)
    (:`NewEnumerator0`
      (set `self.MainWeapon` null))
    (:`NewEnumerator1`
      (set `self.SecondWeapon` null))
    (:`NewEnumerator2`
      (`KismetArrayLibrary.Array_Add` (`self.Specials`)))
    (:`NewEnumerator3`
      (`KismetArrayLibrary.Array_Add` (`self.Grenades`)))
    (:`NewEnumerator4`
      (set `self.MeleeWeapon` null))))

(fn `CreateInventoryType`
  (params (NewWeapon :type "/Game/Blueprints/Weapons/BP_Weapon Object Reference"))
  (set `self.InventoryType` (`|MakeArray` (`/Game/Blueprints/Weapons/BP_Weapon.weaponType` NewWeapon))))

(fn `CreateWeapon`
  (params (Class :type "/Game/Blueprints/Weapons/BP_Weapon Object Reference"))
  (returns (Weapon :type "/Game/Blueprints/Weapons/BP_Weapon Object Reference"))
  (locals (L_Weapon :type "/Game/Blueprints/Weapons/BP_Weapon Object Reference") (NewLocalVar_0 :type "/Game/Blueprints/Weapons/BP_Weapon Object Reference")))

(fn `DefaultWeapon`
  (params (Type :type "/Game/Data/E_WeaponType Enum" :default "NewEnumerator0"))
  (returns (DefaultWeapon :type "/Game/Blueprints/Weapons/BP_Weapon Object Reference"))
  (bind _currentweapon (`self.SelectWeapon` Type))
  (return _currentweapon))

(fn `DeleteTypeInInventory`
  (params (Weapon :type "/Game/Blueprints/Weapons/BP_Weapon Object Reference"))
  (bind _inventorytype (`self.InventoryType`))
  (`KismetArrayLibrary.Array_Remove` _inventorytype (`KismetArrayLibrary.Array_Find` _inventorytype (`/Game/Blueprints/Weapons/BP_Weapon.weaponType` Weapon))))

(fn `DropWeapon`
  (returns (Success :type Boolean))
  (bind _ownerweaponmanager (`self.OwnerWeaponManager`))
  (`Actor.K2_SetActorLocationAndRotation` (`self.CurrentWeapon`) (+ (`Actor.K2_GetActorLocation` _ownerweaponmanager) (* (`Actor.GetActorForwardVector` _ownerweaponmanager) 50.0)) (`Actor.K2_GetActorRotation` _ownerweaponmanager) false false)
  (return true))

(fn `ScrollWeapon`
  (params (Scroll :type Boolean))
  (returns (CurrentWeapon :type "/Game/Blueprints/Weapons/BP_Weapon Object Reference"))
  (bind _inventorytype (`self.InventoryType`))
  (bind _returnvalue (`KismetArrayLibrary.Array_Find` _inventorytype (`/Game/Blueprints/Weapons/BP_Weapon.weaponType` (`self.CurrentWeapon`))))
  (bind _returnvalue_2 (- _returnvalue 1))
  (bind _returnvalue_3 (+ _returnvalue 1))
  (if (> (`KismetArrayLibrary.Array_Length` (`self.InventoryType`)) 0)
    (`self.HiddenWeaponAll` (`self.CurrentWeapon`))
    ;[1 1 1] убрал ShowWeaponOnServer (удалил данную функцию)
    (bind _currentweapon (`self.SelectWeapon` (`|GetArrayItem` (`self.InventoryType`) (`KismetMathLibrary.SelectInt` (`KismetMathLibrary.SelectInt` _returnvalue_3 _returnvalue (< _returnvalue_3 (`KismetArrayLibrary.Array_Length` _inventorytype))) (`KismetMathLibrary.SelectInt` _returnvalue_2 0 (> _returnvalue_2 0)) Scroll))))))

(fn `SelectWeapon`
  (params (Type :type "/Game/Data/E_WeaponType Enum" :default "NewEnumerator0") (Index :type Integer) (WeaponFind :type "/Game/Blueprints/Weapons/BP_Weapon Object Reference"))
  (returns (CurrentWeapon :type "/Game/Blueprints/Weapons/BP_Weapon Object Reference"))
  (if (`KismetArrayLibrary.Array_Contains` (`self.InventoryType`) Type)
    (bind _output_get (set `self.CurrentWeapon` (select `/Game/Data/E_WeaponType` Type :`NewEnumerator0` (`self.MainWeapon`) :`NewEnumerator1` (`self.SecondWeapon`) :`NewEnumerator2` (`|GetArrayItem` (`self.Specials`) Index) :`NewEnumerator3` (`|GetArrayItem` (`self.Grenades`) Index) :`NewEnumerator4` (`self.MeleeWeapon`) :!type "/Game/Blueprints/Weapons/BP_Weapon Object Reference")))
    (return _output_get)))

(fn `SetNewWeaponInInventory`
  (params (NewWeapon :type "/Game/Blueprints/Weapons/BP_Weapon Object Reference"))
  (bind _inventory (`self.Inventory`))
  (switch `/Game/Data/E_WeaponType` (`/Game/Blueprints/Weapons/BP_Weapon.weaponType` NewWeapon)
    (:`NewEnumerator0`
      (`KismetArrayLibrary.Array_Set` _inventory 0 NewWeapon))
    (:`NewEnumerator1`
      (`KismetArrayLibrary.Array_Set` _inventory 1 NewWeapon))
    (:`NewEnumerator2`
      (`KismetArrayLibrary.Array_Set` _inventory 2 NewWeapon))
    (:`NewEnumerator3`
      (`KismetArrayLibrary.Array_Set` _inventory 3 NewWeapon))
    (:`NewEnumerator4`
      (`KismetArrayLibrary.Array_Set` _inventory 4 NewWeapon))))

(fn `SwitchWeapon`
  (params (Weapon :type "/Game/Blueprints/Weapons/BP_Weapon Object Reference")))