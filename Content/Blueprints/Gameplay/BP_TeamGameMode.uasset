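; Team game mode that spawns players inside the start area of their team, red or blue.
; SetStartTrigger caches the bounds of both teams' start actors.
; SpawnPlayer destroys any spectator, spawns a BP_PlayerCharacter at a random XY point in the bounds matching the player state's team, leaving Z unset, then possesses it and marks the player alive.
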(event `self.SetStartTrigger`
  (params (StartRed :type "TriggerBox Object Reference") (StartBlue :type "TriggerBox Object Reference") (StartDeathMatch :type "TriggerBox Object Reference"))
  (bind (_origin _boxextent) (`self.GetActorBounds` StartBlue false))
  (bind (_origin_2 _boxextent_2) (`self.GetActorBounds` StartRed false))
  (`|ExecutionSequence`
    (:`then_0`
      (set `self.RedOrigin` _origin_2)
      (set `self.RedBoxExtent` _boxextent_2))
    (:`then_1`
      (set `self.BlueOrigin` _origin)
      (set `self.BlueBoxExtent` _boxextent))))

(fn `SpawnPlayer`
  (params (PlayerController :type "/Game/Blueprints/Characters/BP_PlayerController Object Reference") (Spectator :type "Pawn Object Reference") (PawnTransform :type "Transform Structure"))
  (returns (SpawnedPlayer :type "/Game/Blueprints/Characters/BP_PlayerCharacter Object Reference"))
  (locals (L_Spectator :type "Pawn Object Reference"))
  (bind _team (`/Game/Blueprints/Characters/BP_TeamPlayerState.team` (cast `/Game/Blueprints/Characters/BP_TeamPlayerState` (`Controller.PlayerState` PlayerController) :!pure true)))
  (bind (_returnvalue_x _returnvalue_y) (`KismetMathLibrary.BreakVector` (`KismetMathLibrary.RandomPointInBoundingBox` (select `/Game/Data/E_Team` _team :`NewEnumerator5` (`self.RedOrigin`) :`NewEnumerator6` (`self.BlueOrigin`)) (select `/Game/Data/E_Team` _team :`NewEnumerator5` (`self.RedBoxExtent`) :`NewEnumerator6` (`self.BlueBoxExtent`)))))
  (bind _output_get (set `local.L_Spectator` Spectator))
  (`/Engine/EditorBlueprintResources/StandardMacros.IsValid` _output_get
    (:`Is Valid`
      (`self.K2_DestroyActor` (`local.L_Spectator`)))
    (:`Is Not Valid`
      _))
  (bind _returnvalue (`|SpawnActorFromClass` "/Game/Blueprints/Characters/BP_PlayerCharacter.BP_PlayerCharacter_C" (`KismetMathLibrary.MakeTransform` (`KismetMathLibrary.MakeVector` _returnvalue_x _returnvalue_y)) "Undefined" "OverrideRootScale" PlayerController null))
  (`Controller.Possess` PlayerController _returnvalue)
  (set `/Game/Blueprints/Characters/BP_PlayerState.Alive` true (cast `/Game/Blueprints/Characters/BP_PlayerState` (`Controller.PlayerState` PlayerController) :!pure true))
  (return null))

(fn `UserConstructionScript`
  (`parent.UserConstructionScript`))