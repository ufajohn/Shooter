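; Game state Blueprint that runs the round clock and relays round and weapon-drop events to clients.
; On authority, BeginPlay starts the match through the game mode, starts a one-second looping countdown and assigns time-up and kill-limit handlers that only print the reason.
; Multicast events fire round start/end dispatchers and place dropped weapons ahead of characters.
; The round-stop handler's binding and most of DropWeapon's inventory cleanup are unconnected.
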(event `self.ReceiveBeginPlay`
  (`/Engine/EditorBlueprintResources/ActorMacros.Switch Has Authority`
    (:`Authority`
      (`GameMode.StartMatch` (`/Game/Blueprints/Libs/BP_FunctionsGlobalGetters.GetBP_GameMode`))
      (`self.StartTimeRound`)
      (add `/Game/Blueprints/Gameplay/BP_GameMode.EndTimeRound` (`/Game/Blueprints/Libs/BP_FunctionsGlobalGetters.GetBP_GameMode`) (delegate `EndTimeRound_Event_0`))
      (add `/Game/Blueprints/Gameplay/BP_GameMode.KillLimitReason` (`/Game/Blueprints/Libs/BP_FunctionsGlobalGetters.GetBP_GameMode`) (delegate `KillLimitReason_Event_0`)))))

(event `EndTimeRound_Event_0`
  (params (Reason :type String))
  (`KismetSystemLibrary.PrintString` Reason))

(event `KillLimitReason_Event_0`
  (params (Reason :type String))
  (`KismetSystemLibrary.PrintString` Reason))

(event `GameStopRound_Event_0`
  (params (Reason :type String))
  (`self.EndRoundMulticast` Reason)
  (`self.StopTimeRound`)
  (set `self.roundInProgress` "NewEnumerator0"))

(event `StartRoundMulticast`
  (`self.StartRound`))

(event `DropWeaponMulticast`
  (params (Character :type "/Game/Blueprints/Characters/BP_PlayerCharacter Object Reference") (DropWeapon :type "/Game/Blueprints/Weapons/BP_Weapon Object Reference"))
  (`self.DropWeapon` Character DropWeapon))

(event `EndRoundMulticast`
  (params (Reason :type String))
  (`self.EndRound` Reason))

(event `DropAllWeaponMulticast`
  (params (Character :type "/Game/Blueprints/Characters/BP_PlayerCharacter Object Reference") (DropWeapon :type "/Game/Blueprints/Weapons/BP_Weapon Object Reference"))
  (`self.DropAllWeapon` Character DropWeapon))

(fn `DropAllWeapon`
  (params (InputPin :type "Actor Object Reference") (InputPin1 :type "/Game/Blueprints/Weapons/BP_Weapon Object Reference"))
  (`self.K2_SetActorLocationAndRotation` (+ (`self.K2_GetActorLocation` InputPin) (* (`self.GetActorForwardVector` InputPin) 50.0)))
  (`/Engine/EditorBlueprintResources/ActorMacros.Switch Has Authority`
    (:`Authority`
      (set `/Game/Blueprints/Weapons/BP_Weapon.WeaponOwner` null InputPin1))))

(fn `DropWeapon`
  (params (L_Character :type "/Game/Blueprints/Characters/BP_PlayerCharacter Object Reference") (DropWeapon :type "/Game/Blueprints/Weapons/BP_Weapon Object Reference"))
  (bind _l_character (`self.L_Character`))
  (set `self.L_Character` L_Character)
  (set `self.L_DropWeapon` DropWeapon)
  (`self.K2_SetActorLocationAndRotation` :`self` (`self.L_DropWeapon`) :`NewLocation` (+ (`self.K2_GetActorLocation` _l_character) (* (`self.GetActorForwardVector` _l_character) 50.0)))
  (`self.SetActorHiddenInGame` (`self.L_DropWeapon`) false)
  (`/Engine/EditorBlueprintResources/ActorMacros.Switch Has Authority`))

(fn `StartTimeRound`
  (set `self.timeRound` (struct))
  (bind _returnvalue (`KismetSystemLibrary.K2_SetTimer` null "TimeTick" 1.0 true))
  (set `self.timerRound` _returnvalue))

(fn `StopTimeRound`
  (`KismetSystemLibrary.K2_ClearAndInvalidateTimerHandle` (`self.timerRound`)))

(fn `TimeTick`
  (bind _output_get (set `self.timeRound` (- (`self.timeRound`) (`KismetMathLibrary.MakeTimespan` 0 0 0 1))))
  (if (and (<= _output_get (`KismetMathLibrary.MakeTimespan` 0)) (`|EnumEquality` (`self.roundInProgress`) "NewEnumerator1"))
    (`self.EndTimeRound` "Время раунда закончилось")))

(fn `UserConstructionScript`)