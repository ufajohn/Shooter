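; Base HUD that switches the player's screen between game HUD, tab and spectator widgets.
; BeginPlay shows the game HUD; ToggleHUD swaps it with the tab widget, and ToggleSpectator swaps it with the spectator view, lazily creating and reusing widgets.
; Death and round-stop handlers show the spectator view, with killer info on death, and the alive handler restores the HUD.
; The code binding these handlers to GameState and PlayerState is disconnected here.
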(event `OnStartRound`)

(event `self.ReceiveBeginPlay`
  (`self.ToggleHUD` false))

(event `GameStopRound_Event_0`
  (params (Reason :type String))
  (`self.ToggleSpectator` true))

(event `OnPlayerAlive`
  (`self.ToggleSpectator` false))

(event `OnPlayerDeath`
  (params (Instigator :type "/Game/Blueprints/Characters/BP_PlayerCharacter Object Reference") (Causer :type "Actor Object Reference"))
  (`self.ToggleSpectator` true)
  (`/Game/Blueprints/UI/Spectator/W_Spectator.Set_Killer_Info` (`self.SpectatorWidget`) Instigator Causer))

(fn `ToggleHUD`
  (params (ShowTab :type Boolean))
  (if ShowTab
    (bind _gamehudwidget (`self.GameHUDWidget`)
      (:`then`
        (`Widget.RemoveFromParent` _gamehudwidget))
      (:`else`
        _))
    (bind _tabwidget (`self.TabWidget`)
      (:`then`
        (`UserWidget.AddToViewport` _tabwidget 0))
      (:`else`
        (bind _returnvalue (`|CreateWidget` (`self.TabWidgetClass`) (`self.GetOwningPlayerController`)))
        (bind _output_get (set `self.TabWidget` _returnvalue))
        (`UserWidget.AddToViewport` _output_get 0)))
    (else
      (bind _tabwidget_2 (`self.TabWidget`)
        (:`then`
          (`Widget.RemoveFromParent` _tabwidget_2))
        (:`else`
          _))
      (bind _gamehudwidget_2 (`self.GameHUDWidget`)
        (:`then`
          (`UserWidget.AddToViewport` _gamehudwidget_2 0))
        (:`else`
          (bind _returnvalue_2 (`|CreateWidget` (`self.GameHUDClass`) (`self.GetOwningPlayerController`)))
          (bind _output_get_2 (set `self.GameHUDWidget` _returnvalue_2))
          (`UserWidget.AddToViewport` _output_get_2 0))))))

(fn `ToggleSpectator`
  (params (Show :type Boolean))
  (if Show
    (bind _gamehudwidget (`self.GameHUDWidget`)
      (:`then`
        (`Widget.RemoveFromParent` _gamehudwidget))
      (:`else`
        _))
    (bind _spectatorwidget (`self.SpectatorWidget`)
      (:`then`
        (`Widget.RemoveFromParent` _spectatorwidget)
        (`UserWidget.AddToViewport` _spectatorwidget 0))
      (:`else`
        (bind _returnvalue (`|CreateWidget` (`self.SpectatorWidgetClass`) (`self.GetOwningPlayerController`)))
        (bind _output_get (set `self.SpectatorWidget` _returnvalue))
        (`UserWidget.AddToViewport` _output_get 0)))
    (else
      (bind _spectatorwidget_2 (`self.SpectatorWidget`)
        (:`then`
          (`Widget.RemoveFromParent` _spectatorwidget_2)
          (`UserWidget.AddToViewport` (`self.GameHUDWidget`) 0))
        (:`else`)))))

(fn `UserConstructionScript`)