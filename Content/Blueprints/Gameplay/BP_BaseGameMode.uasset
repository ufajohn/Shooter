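; Base game mode for a round-based deathmatch with kill scoring, spectating and timed respawns.
; After a short delay it spawns each player at a random XY within the deathmatch trigger's bounds.
; Deaths update scores, drop weapons and possess a spectator following the killer, then respawn the victim while the round runs.
; Reaching the kill limit fires a dispatcher, though its StopRound binding never runs; StopRound moves players to spectators.
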(event `self.ReceiveBeginPlay`
  (`KismetSystemLibrary.Delay` 2.0)
  (`self.StartRound`))

(event `EndTimeRound_Event_0`
  (params (Reason :type String))
  (`self.StopRound` Reason))

(event `EndRoundByKill` :!signature `self.KillLimitReason`
  (params (Reason :type String))
  (`self.StopRound` Reason))

(event `SetStartTrigger`
  (params (StartRed :type "TriggerBox Object Reference") (StartBlue :type "TriggerBox Object Reference") (StartDeathMatch :type "TriggerBox Object Reference"))
  (set `self.startRed` StartRed)
  (set `self.startBlue` StartBlue)
  (set `self.deathMatchTrigger` StartDeathMatch))

(event `RespawnPlayer`
  (params (DeathController :type "/Game/Blueprints/Characters/BP_PlayerController Object Reference") (Spectator :type "Pawn Object Reference"))
  (`KismetSystemLibrary.Delay` (`self.TimeSpawn`))
  (`self.SpawnPlayer` DeathController Spectator))

(fn `CharacterDeath`
  (params (DeathCharacter :type "/Game/Blueprints/Characters/BP_PlayerCharacter Object Reference") (DeathInstigator :type "/Game/Blueprints/Characters/BP_PlayerController Object Reference") (Causer :type "Actor Object Reference"))
  (bind _deathcontroller (`self.deathController`))
  (set `self.DeathCharacter` DeathCharacter)
  (set `self.InstigatorController` DeathInstigator)
  (set `self.Causer` Causer)
  (set `self.InstigatorPawn` (`Controller.K2_GetPawn` (`self.InstigatorController`)))
  (if (`Pawn.IsControlled` (`self.DeathCharacter`))
    (set `self.deathController` (cast `/Game/Blueprints/Characters/BP_PlayerController` (`Pawn.GetController` (`self.DeathCharacter`)) :!pure true))
    (`|ExecutionSequence`
      (:`then_0`
        (`self.UpdateGamePoints` (`self.InstigatorController`) (`self.deathController`)))
      (:`then_1`
        (`self.CharacterDead` (`self.DeathCharacter`) (`self.InstigatorController`) (`self.Causer`))
        (`/Game/Blueprints/Characters/BP_PlayerState.CharDead` (cast `/Game/Blueprints/Characters/BP_PlayerState` (`Pawn.PlayerState` (`self.DeathCharacter`)) :!pure true) (cast `/Game/Blueprints/Characters/BP_PlayerCharacter` (`self.InstigatorPawn`) :!pure true) (`self.Causer`)))
      (:`then_2`
        (for _array_element (`/Game/Blueprints/Components/BP_WeaponManager.Inventory` (`/Game/Blueprints/Characters/BP_PlayerCharacter.BP_WeaponManager` (`self.DeathCharacter`)))
          (`/Engine/EditorBlueprintResources/StandardMacros.IsValid` _array_element
            (:`Is Valid`
              (`/Game/Blueprints/Gameplay/BP_GameStateBase.DropAllWeaponMulticast` (cast `/Game/Blueprints/Gameplay/BP_GameStateBase` (`GameplayStatics.GetGameState`) :!pure true) (`self.DeathCharacter`) _array_element))))
        (`KismetSystemLibrary.K2_SetTimer` (`self.DeathCharacter`) "K2_DestroyActor" (`self.TimeSpawn`)))
      (:`then_3`
        (if (>= (`/Game/Blueprints/Characters/BP_PlayerState.killPoints` (cast `/Game/Blueprints/Characters/BP_PlayerState` (`Controller.PlayerState` (`self.InstigatorController`)) :!pure true)) (`self.killsLimit`))
          (`self.KillLimitReason` "Достигнут лимит убийств")
          (else
            (`self.SpawnSpectator` (`self.InstigatorController`) (`self.deathController`))
            (if (`|EnumEquality` (`/Game/Blueprints/Gameplay/BP_GameStateBase.roundInProgress` (`/Game/Blueprints/Libs/BP_FunctionsGlobalGetters.GetBP_BaseGameState`)) "NewEnumerator1")
              (`self.RespawnPlayer` _deathcontroller (`Controller.K2_GetPawn` _deathcontroller)))))))))

(fn `SpawnPlayer`
  (params (PlayerController :type "/Game/Blueprints/Characters/BP_PlayerController Object Reference") (Spectator :type "Pawn Object Reference") (PawnTransform :type "Transform Structure"))
  (returns (SpawnedPlayer :type "/Game/Blueprints/Characters/BP_PlayerCharacter Object Reference"))
  (locals (L_Spectator :type "Pawn Object Reference"))
  (bind (_origin _boxextent) (`self.GetActorBounds` (`self.deathMatchTrigger`) false))
  (bind (_returnvalue_x _returnvalue_y) (`KismetMathLibrary.BreakVector` (`KismetMathLibrary.RandomPointInBoundingBox` _origin _boxextent)))
  (bind _output_get (set `local.L_Spectator` Spectator))
  (`/Engine/EditorBlueprintResources/StandardMacros.IsValid` _output_get
    (:`Is Valid`
      (`self.K2_DestroyActor` (`local.L_Spectator`)))
    (:`Is Not Valid`
      _))
  (bind _returnvalue (`|SpawnActorFromClass` "/Game/Blueprints/Characters/BP_PlayerCharacter.BP_PlayerCharacter_C" (`KismetMathLibrary.MakeTransform` (`KismetMathLibrary.MakeVector` _returnvalue_x _returnvalue_y)) "Undefined" "OverrideRootScale" PlayerController null))
  (`Controller.Possess` PlayerController _returnvalue)
  (set `/Game/Blueprints/Characters/BP_PlayerState.Alive` true (cast `/Game/Blueprints/Characters/BP_PlayerState` (`Controller.PlayerState` PlayerController) :!pure true))
  (return _returnvalue))

(fn `SpawnSpectator`
  (params (`Death Instigator` :type "/Game/Blueprints/Characters/BP_PlayerController Object Reference") (`Death Controller` :type "/Game/Blueprints/Characters/BP_PlayerController Object Reference"))
  (returns (Spectator :type "Pawn Object Reference"))
  (locals (L_Pawn :type "Pawn Object Reference") (L_Controller :type "/Game/Blueprints/Characters/BP_PlayerController Object Reference"))
  (bind _returnvalue (`Controller.K2_GetPawn` (`local.L_Controller`)))
  (set `local.L_Controller` `Death Controller`)
  (`/Engine/EditorBlueprintResources/StandardMacros.IsValid` `Death Instigator`
    (:`Is Valid`
      (bind _returnvalue_2 (`|SpawnActorFromClass` "/Game/Blueprints/Characters/BP_SpectatorPawnFollow.BP_SpectatorPawnFollow_C" (`self.GetTransform` (`Controller.K2_GetPawn` (`self.deathController`))) "Undefined" "OverrideRootScale" (`self.deathController`) null))
      (`Controller.Possess` (`self.deathController`) _returnvalue_2)
      (set `/Game/Blueprints/Characters/BP_SpectatorPawnFollow.followCharacter` (cast `/Game/Blueprints/Characters/BP_PlayerCharacter` (`self.InstigatorPawn`) :!pure true) _returnvalue_2)
      (return _returnvalue_2))
    (:`Is Not Valid`
      (set `local.L_Pawn` _returnvalue)
      (bind _returnvalue_3 (`|SpawnActorFromClass` "/Game/Blueprints/Characters/BP_SpectatorPawnFree.BP_SpectatorPawnFree_C" (`self.GetTransform` _returnvalue) "Undefined" "OverrideRootScale" (`local.L_Controller`) null))
      (`Controller.Possess` (`local.L_Controller`) _returnvalue_3)
      (set `/Game/Blueprints/Characters/BP_SpectatorPawnFree.FreeSpectator` (cast `/Game/Blueprints/Characters/BP_PlayerCharacter` (`local.L_Pawn`) :!pure true) _returnvalue_3)
      (return _returnvalue_3))))

(fn `StartRound`
  (bind _asbp_game_state_base (cast `/Game/Blueprints/Gameplay/BP_GameStateBase` (`GameplayStatics.GetGameState`)))
  (for _array_element (`GameStateBase.PlayerArray` _asbp_game_state_base)
    (bind _asbp_player_controller (cast `/Game/Blueprints/Characters/BP_PlayerController` (`self.GetOwner` _array_element)))
    (`self.SpawnPlayer` _asbp_player_controller))
  (`self.GameStartRound`))

(fn `StopRound`
  (params (Reason :type String))
  (`KismetSystemLibrary.PrintString` Reason true true (struct :`G` 0.66 :`B` 1.0 :`A` 1.0) 60.0)
  (for _array_element (`GameStateBase.PlayerArray` (`GameplayStatics.GetGameState`))
    (bind _asbp_player_controller (cast `/Game/Blueprints/Characters/BP_PlayerController` (`self.GetOwner` _array_element)))
    (if (== _asbp_player_controller (`self.deathController`))
      (`self.SpawnSpectator` (`self.InstigatorController`) (`self.deathController`))
      (else
        (`self.SpawnSpectator` null _asbp_player_controller))))
  (`self.GameStopRound` Reason))

(fn `UpdateGamePoints`
  (params (DeathInstigator :type "/Game/Blueprints/Characters/BP_PlayerController Object Reference") (DeathController :type "/Game/Blueprints/Characters/BP_PlayerController Object Reference"))
  (`/Game/Blueprints/Characters/BP_PlayerState.AddKillPoints` (cast `/Game/Blueprints/Characters/BP_PlayerState` (`Controller.PlayerState` DeathInstigator) :!pure true))
  (`/Game/Blueprints/Characters/BP_PlayerState.AddDeathPoints` (cast `/Game/Blueprints/Characters/BP_PlayerState` (`Controller.PlayerState` DeathController) :!pure true)))

(fn `UserConstructionScript`)