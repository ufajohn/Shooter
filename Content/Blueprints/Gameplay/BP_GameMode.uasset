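; Deathmatch game mode that starts the match after a short delay and handles kills, spectating and respawns.
; CharacterDeath updates kill/death points, drops weapons via GameState multicast and possesses the victim into a spectator pawn.
; It then either signals the kill limit or, after a delay, respawns the player at a random point within DeathMatchTrigger bounds.
; Login, logout, match-state and StopRound entry points are empty, their logic left disconnected.
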(event `self.ReceiveBeginPlay`
  (`KismetSystemLibrary.Delay` 2.0)
  (`self.StartMatch`))

(event `self.K2_PostLogin`
  (params (NewPlayer :type "PlayerController Object Reference"))
  ;[1 1 1] Handle Login and Logout
)

(event `SetStartTrigger`
  (params (StartRed :type "TriggerBox Object Reference") (StartBlue :type "TriggerBox Object Reference") (StartDeathMatch :type "TriggerBox Object Reference")))

(event `self.K2_OnSwapPlayerControllers`
  (params (OldPC :type "PlayerController Object Reference") (NewPC :type "PlayerController Object Reference"))
  ;[1 1 1] Handle Login and Logout
  (bind _asbp_game_state (cast `/Game/Blueprints/Gameplay/BP_GameState` (`GameplayStatics.GetGameState`)))
  (`/Game/Blueprints/Gameplay/BP_GameState.AddPlayer` _asbp_game_state null)
  (bind _asbp_player_controller (cast `/Game/Blueprints/Characters/BP_PlayerController` NewPC))
  (`/Game/Blueprints/Characters/BP_PlayerController.InitialSetup` _asbp_player_controller))

(event `RespawnPlayer`
  (params (DeathController :type "/Game/Blueprints/Characters/BP_PlayerController Object Reference") (Spectator :type "Pawn Object Reference"))
  (`KismetSystemLibrary.Delay` (`self.TimeSpawn`))
  (`self.SpawnPlayer` DeathController Spectator))

(event `self.K2_OnLogout`
  (params (ExitingController :type "Controller Object Reference"))
  ;[1 1 1] Handle Login and Logout
)

(event `CustomEvent_1`
  (params (StartRed :type "TriggerBox Object Reference") (StartBlue :type "TriggerBox Object Reference") (StartDeathMatch :type "TriggerBox Object Reference")))

(event `CustomEvent`
  (params (NewState :type Name))
  ;[1 1 1] On Match State Changed
)

(event `EndTimeRound_Event_0`
  (params (Reason :type String))
  (`self.StopRound` Reason))

(event `EndRoundByKill` :!signature `self.KillLimitReason`
  (params (Reason :type String))
  (`self.StopRound` Reason))

(fn `CharacterDeath`
  (params (DeathCharacter :type "/Game/Blueprints/Characters/BP_PlayerCharacter Object Reference") (Instigator :type "/Game/Blueprints/Characters/BP_PlayerController Object Reference") (Causer :type "Actor Object Reference"))
  (bind _deathcontroller (`self.deathController`))
  (set `self.DeathCharacter` DeathCharacter)
  (set `self.InstigatorController` Instigator)
  (set `self.Causer` Causer)
  (set `self.InstigatorPawn` (`Controller.K2_GetPawn` (`self.InstigatorController`)))
  (if (`Pawn.IsControlled` (`self.DeathCharacter`))
    (set `self.deathController` (cast `/Game/Blueprints/Characters/BP_PlayerController` (`Pawn.GetController` (`self.DeathCharacter`)) :!pure true))
    (`|ExecutionSequence`
      (:`then_0`
        (`self.UpdateGamePoints` (`self.InstigatorController`) (`self.deathController`)))
      (:`then_1`
        (`self.CharacterDead` (`self.DeathCharacter`) (`self.InstigatorController`) (`self.Causer`)))
      (:`then_2`
        (for _array_element (`/Game/Blueprints/Components/BP_WeaponManager.Inventory` (`/Game/Blueprints/Characters/BP_PlayerCharacter.BP_WeaponManager` (`self.DeathCharacter`)))
          (`/Engine/EditorBlueprintResources/StandardMacros.IsValid` _array_element
            (:`Is Valid`
              (`/Game/Blueprints/Gameplay/BP_GameState.DropAllWeaponMulticast` (cast `/Game/Blueprints/Gameplay/BP_GameState` (`GameplayStatics.GetGameState`) :!pure true) (`self.DeathCharacter`) _array_element)
              (`KismetSystemLibrary.K2_SetTimer` (`self.DeathCharacter`) "K2_DestroyActor" (`self.TimeSpawn`) :!label _label))))
        (goto _label))
      (:`then_3`
        (if (>= (`/Game/Blueprints/Characters/BP_PlayerState.killPoints` (cast `/Game/Blueprints/Characters/BP_PlayerState` (`Controller.PlayerState` (`self.InstigatorController`)) :!pure true)) (`self.killsLimit`))
          (`self.SpawnSpectator` (`self.InstigatorController`) (`self.deathController`))
          (`self.KillLimitReason` "Достигнут лимит убийств")
          (else
            (`self.SpawnSpectator` (`self.InstigatorController`) (`self.deathController`))
            (`self.RespawnPlayer` _deathcontroller (`Controller.K2_GetPawn` _deathcontroller))))))))

(fn `SpawnPlayer`
  (params (PlayerController :type "/Game/Blueprints/Characters/BP_PlayerController Object Reference") (Spectator :type "Pawn Object Reference"))
  (returns (SpawnedPlayer :type "/Game/Blueprints/Characters/BP_PlayerCharacter Object Reference"))
  (bind (_origin _boxextent) (`self.GetActorBounds` (`self.deathMatchTrigger`) false))
  (bind (_returnvalue_x _returnvalue_y) (`KismetMathLibrary.BreakVector` (`KismetMathLibrary.RandomPointInBoundingBox` _origin _boxextent)))
  (bind _output_get (set `self.L_Spectator` Spectator))
  (`/Engine/EditorBlueprintResources/StandardMacros.IsValid` _output_get
    (:`Is Valid`
      (`self.K2_DestroyActor` (`self.L_Spectator`)))
    (:`Is Not Valid`
      _))
  (bind _returnvalue (`|SpawnActorFromClass` "/Game/Blueprints/Characters/BP_PlayerCharacter.BP_PlayerCharacter_C" (`KismetMathLibrary.MakeTransform` (`KismetMathLibrary.MakeVector` _returnvalue_x _returnvalue_y)) "Undefined" "OverrideRootScale" PlayerController null))
  (`Controller.Possess` PlayerController _returnvalue)
  (set `/Game/Blueprints/Characters/BP_PlayerState.Alive` true (cast `/Game/Blueprints/Characters/BP_PlayerState` (`Controller.PlayerState` PlayerController) :!pure true))
  (return _returnvalue))

(fn `SpawnSpectator`
  (params (DeathInstigator :type "/Game/Blueprints/Characters/BP_PlayerController Object Reference") (L_Controller :type "/Game/Blueprints/Characters/BP_PlayerController Object Reference"))
  (returns (Spectator :type "Pawn Object Reference"))
  (bind _returnvalue (`Controller.K2_GetPawn` (`self.L_Controller`)))
  (set `self.L_Controller` L_Controller)
  (`/Engine/EditorBlueprintResources/StandardMacros.IsValid` DeathInstigator
    (:`Is Valid`
      (bind _returnvalue_2 (`|SpawnActorFromClass` "/Game/Blueprints/Characters/BP_SpectatorPawnFollow.BP_SpectatorPawnFollow_C" (`self.GetTransform` (`Controller.K2_GetPawn` (`self.deathController`))) "Undefined" "OverrideRootScale" (`self.deathController`) null))
      (`Controller.Possess` (`self.deathController`) _returnvalue_2)
      (set `/Game/Blueprints/Characters/BP_SpectatorPawnFollow.followCharacter` (cast `/Game/Blueprints/Characters/BP_PlayerCharacter` (`self.GetInstigator`) :!pure true) _returnvalue_2)
      (return _returnvalue_2))
    (:`Is Not Valid`
      (set `self.L_Pawn` _returnvalue)
      (bind _returnvalue_3 (`|SpawnActorFromClass` "/Game/Blueprints/Characters/BP_SpectatorPawnFree.BP_SpectatorPawnFree_C" (`self.GetTransform` _returnvalue) "Undefined" "OverrideRootScale" (`self.L_Controller`) null))
      (`Controller.Possess` (`self.L_Controller`) _returnvalue_3)
      (set `/Game/Blueprints/Characters/BP_SpectatorPawnFree.FreeSpectator` (cast `/Game/Blueprints/Characters/BP_PlayerCharacter` (`self.L_Pawn`) :!pure true) _returnvalue_3)
      (return _returnvalue_3))))

(fn `StopRound`
  (params (Reason :type String)))

(fn `UpdateGamePoints`
  (params (InstigatorController :type "/Game/Blueprints/Characters/BP_PlayerController Object Reference") (DeathController :type "/Game/Blueprints/Characters/BP_PlayerController Object Reference"))
  (`/Game/Blueprints/Characters/BP_PlayerState.AddKillPoints` (cast `/Game/Blueprints/Characters/BP_PlayerState` (`Controller.PlayerState` InstigatorController) :!pure true))
  (`/Game/Blueprints/Characters/BP_PlayerState.AddDeathPoints` (cast `/Game/Blueprints/Characters/BP_PlayerState` (`Controller.PlayerState` DeathController) :!pure true)))

(fn `UserConstructionScript`)