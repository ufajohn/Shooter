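; Player controller that sets game-only input on begin play and shows the BP_BaseHUD toggle while Tab is held.
; Dead ragdolls a given character by disabling movement and capsule collision and enabling mesh physics.
; SpawnSpectator is an empty entry point.
; Its disconnected logic would possess a spectator pawn that follows the death instigator's character, or a free one without a valid instigator.
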(event `self.ReceiveBeginPlay`
  (`WidgetBlueprintLibrary.SetInputMode_GameOnly` self))

(event `Key|Tab`
  (params (Key :type "Key Structure"))
  (bind _asbp_base_hud (cast `/Game/Blueprints/Gameplay/BP_BaseHUD` (`self.GetHUD`) :!pure true))
  (:`Pressed`
    (`/Game/Blueprints/Gameplay/BP_BaseHUD.ToggleHUD` _asbp_base_hud true))
  (:`Released`
    (`/Game/Blueprints/Gameplay/BP_BaseHUD.ToggleHUD` _asbp_base_hud false)))

(fn `Dead`
  (params (DeathCharacter :type "/Game/Blueprints/Characters/BP_PlayerCharacter Object Reference"))
  (bind _mesh (`Character.Mesh` DeathCharacter))
  (`CharacterMovementComponent.DisableMovement` (`Character.CharacterMovement` DeathCharacter))
  (`PrimitiveComponent.SetCollisionEnabled` (`Character.CapsuleComponent` DeathCharacter) "NoCollision")
  (`PrimitiveComponent.SetCollisionEnabled` _mesh "QueryAndPhysics")
  (`PrimitiveComponent.SetSimulatePhysics` _mesh true))

(fn `SpawnSpectator`
  (params (DeathInstigator :type "/Game/Blueprints/Characters/BP_PlayerController Object Reference"))
  (returns (Spectator :type "Pawn Object Reference"))
  (locals (L_Pawn :type "Pawn Object Reference")))

(fn `UserConstructionScript`)