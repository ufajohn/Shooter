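; BP_PlayerState is a player state that tracks a player's kill points, death points and alive status.
; CharDead clears Alive and broadcasts PlayerDeath with instigator and causer, while the Alive RepNotify broadcasts PlayerAlive only when it becomes true.
; AddDeathPoints increments deaths and fires a death dispatcher.
; AddKillPoints increments kills and compares them to BP_GameMode's KillsLimit, but that branch leads to no action.
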(event `CharDead`
  (params (Instigator :type "/Game/Blueprints/Characters/BP_PlayerCharacter Object Reference") (Causer :type "Actor Object Reference"))
  (set `self.Alive` false)
  (`self.PlayerDeath` Instigator Causer))

(fn `AddDeathPoints`
  (bind _result (`/Engine/EditorBlueprintResources/StandardMacros.IncrementInt` (`self.deathPoints`))
    (:`  `
      (set `self.deathPoints` _result)
      (`self.DeathDispatcher`))))

(fn `AddKillPoints`
  (bind _result (`/Engine/EditorBlueprintResources/StandardMacros.IncrementInt` (`self.killPoints`))
    (:`  `
      (bind _output_get (set `self.killPoints` _result))
      (if (>= _output_get (`/Game/Blueprints/Gameplay/BP_GameMode.killsLimit` (cast `/Game/Blueprints/Gameplay/BP_GameMode` (`GameplayStatics.GetGameMode`) :!pure true)))
        _))))

(fn `OnRep_Alive`
  (if (`self.Alive`)
    (`self.PlayerAlive`)))

(fn `UserConstructionScript`)