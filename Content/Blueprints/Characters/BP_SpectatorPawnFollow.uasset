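; BP_SpectatorPawnFollow is a spectator pawn that trails a followed character.
; Each Tick, only on the locally controlled client without authority, it eases its location toward a valid FollowCharacter using VInterpTo at InterSpeed, without sweeping.
; It changes location only, and nothing in this file assigns FollowCharacter.
; Two disconnected debug print chains remain in the event graph and never run.
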(event `self.ReceiveBeginPlay`)

(event `self.ReceiveTick`
  (params (DeltaSeconds :type "Float (single-precision)"))
  (if (`self.IsLocallyControlled`)
    (`/Engine/EditorBlueprintResources/ActorMacros.Switch Has Authority`
      (:`Remote`
        (bind _followcharacter (`self.followCharacter`)
          (:`then`
            (`self.K2_SetActorLocation` (`KismetMathLibrary.VInterpTo` (`self.K2_GetActorLocation`) (`self.K2_GetActorLocation` _followcharacter) (`GameplayStatics.GetWorldDeltaSeconds`) (`self.interSpeed`))))
          (:`else`))))))

(fn `UserConstructionScript`)