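; Firearm weapon that plays a gunshot and either spawns a projectile or, without a projectile class, applies point damage through a line trace.
; The trace starts at the player's camera, follows the owner's forward vector and draws debug shapes.
; An empty magazine with reserve ammo sets Reload during a specific round state.
; Reload's OnRep starts an authority-only timer that refills the magazine to its class default from reserves.
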(event `PlaySound`
  (`GameplayStatics.SpawnSoundAtLocation` "/Game/Assets/Sounds/m-16_odinochnye_vystrely.m-16_odinochnye_vystrely" (`self.K2_GetActorLocation` self) (struct) 1.0 1.0 0.0 null null))

(event `DEBUG_DrawServerTrace`
  (params (Start :type "Vector Structure") (End :type "Vector Structure") (Hit :type "Vector Structure"))
  (`KismetSystemLibrary.DrawDebugLine` Start End (struct :`R` 1.0 :`G` 0.692331 :`A` 1.0) 5.0 2.0)
  (`KismetSystemLibrary.DrawDebugSphere` Hit 20.0 8 (struct :`R` 1.0 :`G` 0.076999 :`A` 1.0) 5.0 2.0))

(event `GetProjectileOnAll`)

(fn `AbleToUseWeapon`
  (returns (Out :type Boolean))
  (return (and (`parent.AbleToUseWeapon`) (not (`self.Reload`)))))

(fn `Get_Projectile`
  (`|SpawnActorFromClass` (`self.projectile`) (`/Game/Blueprints/Characters/BP_PlayerCharacter.SpawnTransform` (`self.WeaponOwner`)) "AlwaysSpawn" "OverrideRootScale" self (`self.damage`) (`self.GetInstigator`)))

(fn `GetFireTrace`
  (returns (Hit :type "HitResult Structure"))
  (bind _returnvalue (`self.GetInstigator`))
  (if (`KismetSystemLibrary.IsValid` _returnvalue)
    (bind _asbp_player_character (cast `/Game/Blueprints/Characters/BP_PlayerCharacter` _returnvalue)
      (:`then`
        (bind _returnvalue_2 (`SceneComponent.K2_GetComponentLocation` (`/Game/Blueprints/Characters/BP_PlayerCharacter.FreeCamera` _asbp_player_character)))
        (bind _outhit (`KismetSystemLibrary.LineTraceSingleForObjects` _returnvalue_2 (+ _returnvalue_2 (* (`self.GetActorForwardVector` (`self.GetOwner`)) 10000.0)) (`|MakeArray` "ObjectTypeQuery1" "ObjectTypeQuery2" "ObjectTypeQuery3" :!type "EObjectTypeQuery Enum") false (`|MakeArray` (`self.GetInstigator`) self null :!type "Actor Object Reference") "ForDuration"))
        (bind (_bblockinghit _binitialoverlap _time _distance _location _impactpoint _normal _impactnormal _physmat _hitactor _hitcomponent _hitbonename _hititem _faceindex _tracestart _traceend) (`GameplayStatics.BreakHitResult` _outhit))
        (`self.DEBUG_DrawServerTrace` _tracestart _traceend _location)
        (return _outhit))
      (:`CastFailed`
        (return)))))

(fn `OnRep_Reload`
  (`/Engine/EditorBlueprintResources/ActorMacros.Switch Has Authority`
    (:`Authority`
      (if (`self.Reload`)
        (`KismetSystemLibrary.K2_SetTimer` null "ReloadFinished" 2.0)))))

(fn `ReloadFinished`
  (bind (_projectile _currentammo) (defaults `/Game/Blueprints/Weapons/BP_FireWeapon` "BP_FireWeapon_C"))
  (bind _returnvalue (+ (`self.TotalAmmo`) (`self.CurrentAmmo`)))
  (set `self.Reload` false)
  (if (>= (`self.TotalAmmo`) _currentammo)
    (bind _output_get (set `self.TotalAmmo` (- (`self.TotalAmmo`) (- (`.CurrentAmmo` (defaults `/Game/Blueprints/Weapons/BP_FireWeapon` "BP_FireWeapon_C")) (`self.CurrentAmmo`)))))
    (set `self.CurrentAmmo` _currentammo)
    (`KismetSystemLibrary.PrintString` (`KismetStringLibrary.Concat_StrStr` "магазин перезаряжен, в запасе патронов: " (`KismetStringLibrary.Conv_IntToString` _output_get)) true true (struct :`R` 1.0 :`B` 0.139431 :`A` 1.0) 30.0)
    (elif (<= _returnvalue (`.CurrentAmmo` (defaults `/Game/Blueprints/Weapons/BP_FireWeapon` "BP_FireWeapon_C")))
      (bind _output_get_2 (set `self.CurrentAmmo` _returnvalue))
      (set `self.TotalAmmo` 0)
      (`KismetSystemLibrary.PrintString` (`KismetStringLibrary.Concat_StrStr` "в магазине последние " (`KismetStringLibrary.Conv_IntToString` _output_get_2) " патронов, в запасе нет патронов") true true (struct :`G` 0.109375 :`B` 0.010309 :`A` 1.0) 30.0)
      (else
        (bind _output_get_3 (set `self.TotalAmmo` (- (+ (`self.TotalAmmo`) (`self.CurrentAmmo`)) (`.CurrentAmmo` (defaults `/Game/Blueprints/Weapons/BP_FireWeapon` "BP_FireWeapon_C")))))
        (set `self.CurrentAmmo` (`.CurrentAmmo` (defaults `/Game/Blueprints/Weapons/BP_FireWeapon` "BP_FireWeapon_C")))
        (`KismetSystemLibrary.PrintString` (`KismetStringLibrary.Concat_StrStr` "магазин перезаряжен, в запасе " (`KismetStringLibrary.Conv_IntToString` _output_get_3) " патронов") true true (struct :`G` 0.66 :`B` 1.0 :`A` 1.0) 30.0)))))

(fn `UserConstructionScript`)

(fn `UseWeapon`
  (params (SpawnTransform :type "Transform Structure"))
  (returns (Used :type Boolean))
  (`parent.UseWeapon` SpawnTransform)
  (if (and (> (`self.CurrentAmmo`) 0) (not (`self.Reload`)))
    (`self.PlaySound`)
    (if (`KismetSystemLibrary.IsValidClass` (`self.projectile`))
      (`self.Get_Projectile`)
      (return true)
      (else
        (bind _hit (`self.GetFireTrace`))
        (bind (_bblockinghit _binitialoverlap _time _distance _location _impactpoint _normal _impactnormal _physmat _hitactor _hitcomponent _hitbonename _hititem _faceindex _tracestart _traceend) (`GameplayStatics.BreakHitResult` _hit))
        (`GameplayStatics.ApplyPointDamage` _hitactor (`self.damage`) (`KismetMathLibrary.GetDirectionUnitVector` _traceend _tracestart) _hit (`self.GetInstigatorController`) self)
        (return true)))
    (elif (or (and (> (`self.TotalAmmo`) 0) (<= (`self.CurrentAmmo`) 0)) (and (> (`self.TotalAmmo`) 0) (> (`self.CurrentAmmo`) 0) (`self.Reload`)))
      (if (`|EnumEquality` (`/Game/Blueprints/Gameplay/BP_GameState.roundInProgress` (`/Game/Blueprints/Libs/BP_FunctionsGlobalGetters.GetBP_GameState`)) "NewEnumerator1")
        (`KismetSystemLibrary.PrintString` "запустился процесс перезарядки" true true (struct :`R` 1.0 :`G` 0.910626 :`A` 1.0))
        (set `self.Reload` true)
        (return false))
      (elif (and (<= (`self.TotalAmmo`) 0) (<= (`self.CurrentAmmo`) 0))
        (`KismetSystemLibrary.PrintString` "Патроны закончились")
        (else
          (return false))))))