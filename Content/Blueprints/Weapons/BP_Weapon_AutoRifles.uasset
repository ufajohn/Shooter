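; Weapon Blueprint for automatic rifles, extending a parent weapon class.
; UseWeapon calls the parent implementation, then sets IsAutoFire to true and returns the parent's result.
; The GetProjectile event spawns the projectile class at the weapon owner's spawn transform, always spawning regardless of collision, and passes it the damage, owner and instigator.
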(event `self.Get_Projectile`
  (bind (_spawntransform_location _spawntransform_rotation) (`KismetMathLibrary.BreakTransform` (`/Game/Blueprints/Characters/BP_PlayerCharacter.SpawnTransform` (`self.WeaponOwner`))))
  (`|SpawnActorFromClass` (`self.projectile`) (`KismetMathLibrary.MakeTransform` _spawntransform_location _spawntransform_rotation) "AlwaysSpawn" "OverrideRootScale" self (`self.damage`) (`self.GetInstigator`)))

(fn `UserConstructionScript`
  (`parent.UserConstructionScript`))

(fn `UseWeapon`
  (params (SpawnTransform :type "Transform Structure"))
  (returns (Used :type Boolean))
  (bind _used (`parent.UseWeapon` (struct)))
  (set `self.IsAutoFire` true)
  (return _used))