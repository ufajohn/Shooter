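; Weapon spawner actor that places one random weapon pickup at its location when play begins.
; On BeginPlay, only the authority runs SpawnWeapon, so the server decides the weapon.
; SpawnWeapon picks at random between auto rifle, pistol and knife Blueprints, then spawns it slightly above the root, rolled onto its side with a random yaw, ignoring collisions.
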(event `self.ReceiveBeginPlay`
  (`/Engine/EditorBlueprintResources/ActorMacros.Switch Has Authority`
    (:`Authority`
      (`self.SpawnWeapon`))))

(fn `SpawnWeapon`
  (`|SpawnActorFromClass` (select `int` (`KismetMathLibrary.RandomIntegerInRange` 0 2) :`0` "/Game/Blueprints/Weapons/BP_Weapon_AutoRifles.BP_Weapon_AutoRifles_C" :`1` "/Game/Blueprints/Weapons/BP_Weapon_Pistols.BP_Weapon_Pistols_C" :`2` "/Game/Blueprints/Weapons/BP_Weapon_Knife.BP_Weapon_Knife_C" :!type "/Game/Blueprints/Weapons/BP_Weapon Class Reference") (`KismetMathLibrary.MakeTransform` (`KismetMathLibrary.MakeVector` (.x (`SceneComponent.K2_GetComponentLocation` (`self.DefaultSceneRoot`))) (.y (`SceneComponent.K2_GetComponentLocation` (`self.DefaultSceneRoot`))) (+ (.z (`SceneComponent.K2_GetComponentLocation` (`self.DefaultSceneRoot`))) 2.0)) (`KismetMathLibrary.MakeRotator` 90.0 0.0 (`KismetMathLibrary.RandomFloatInRange` 0.0 360.0))) "AlwaysSpawn" "OverrideRootScale" null null null))

(fn `UserConstructionScript`)