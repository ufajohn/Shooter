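; Weapon actor that can be picked up through Interact, which passes it to the character's BPWeaponManager to add to the inventory on the server.
; OnRep_WeaponOwner sets instigator and owner and attaches it to the mesh's Skt_Weapon socket, or detaches it and restores collision and visibility.
; UseWeapon spends ammo behind a timer-based rate lock and repeats while IsAutoFire is set; it spawns nothing here.
; EventGraph logic is disconnected leftover.
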(event `self.ReceiveBeginPlay`)

(event `self.ReceiveTick`
  (params (DeltaSeconds :type "Float (single-precision)")))

(event `CustomEvent_0`
  (params (owner :type "/Game/Blueprints/Characters/BP_PlayerCharacter Object Reference")))

(fn `AbleToUseWeapon`
  (returns (Out :type Boolean))
  (return (and (> (`self.CurrentAmmo`) 0) (not (`self.UseFreezedByRate`)))))

(fn `Interact`
  (params (Character :type "/Game/Blueprints/Characters/BP_PlayerCharacter Object Reference") (Hit :type "HitResult Structure"))
  (returns (Success :type Boolean))
  (`/Game/Blueprints/Components/BP_WeaponManager.AddWeaponInInventoryOnServer` (`/Game/Blueprints/Characters/BP_PlayerCharacter.BP_WeaponManager` Character) Character self)
  (return true))

(fn `OnRep_WeaponOwner`
  (bind _weaponowner (`self.WeaponOwner`)
    (:`then`
      (set `self.Instigator` _weaponowner)
      (`self.SetOwner` (`Pawn.GetController` _weaponowner))
      (`self.K2_AttachToComponent` (`Character.Mesh` (`self.WeaponOwner`)) "Skt_Weapon" "SnapToTarget" "SnapToTarget" "KeepRelative"))
    (:`else`
      (`self.K2_DetachFromActor` "KeepWorld" "KeepWorld")
      (`self.SetActorEnableCollision` true)
      (`self.SetActorHiddenInGame` false)
      (set `self.Instigator` null)
      (`self.SetOwner` null))))

(fn `StopRateDelay`
  (set `self.UseFreezedByRate` false)
  (if (`self.IsAutoFire`)
    (`self.UseWeapon` (struct))))

(fn `StopUseWeapon`
  (set `self.IsAutoFire` false))

(fn `UserConstructionScript`)

(fn `UseWeapon`
  (params (SpawnTransform :type "Transform Structure"))
  (returns (Used :type Boolean))
  (if (`self.AbleToUseWeapon`)
    (`/Engine/EditorBlueprintResources/StandardMacros.DecrementInt` (`self.CurrentAmmo`)
      (:`  `
        (`KismetSystemLibrary.K2_SetTimer` null "StopRateDelay" (`self.UseRate`))
        (set `self.UseFreezedByRate` true)
        (return true)))
    (else
      (return false))))