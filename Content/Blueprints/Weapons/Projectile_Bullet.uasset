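; Networked bullet projectile actor that deals point damage on hit and leaves bullet-mark decals.
; The server applies a fixed damage to the hit actor and destroys the bullet, while remote instances spawn a randomly sized, temporary decal attached to the struck component.
; An exit-point function meant to trace back toward the hit is left unconnected, with its debug-drawn trace logic never running.
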(event `self.ReceiveHit`
  (params (MyComp :type "PrimitiveComponent Object Reference") (Other :type "Actor Object Reference") (OtherComp :type "PrimitiveComponent Object Reference") (bSelfMoved :type Boolean) (HitLocation :type "Vector Structure") (HitNormal :type "Vector Structure") (NormalImpulse :type "Vector Structure") (Hit :type "HitResult Structure (by ref)"))
  (bind _returnvalue (`KismetMathLibrary.RandomFloatInRange` 6.0 8.0))
  (bind _returnvalue_2 (`SceneComponent.K2_GetComponentToWorld` OtherComp))
  (`/Engine/EditorBlueprintResources/ActorMacros.Switch Has Authority`
    (:`Authority`
      (`GameplayStatics.ApplyPointDamage` Other 10.0 (`self.K2_GetActorLocation`) Hit (`self.GetInstigatorController`) self)
      (`self.K2_DestroyActor`))
    (:`Remote`
      (`GameplayStatics.SpawnDecalAttached` "/Game/Assets/Weapon/bullet-mark-png-12_Mat_Decal.bullet-mark-png-12_Mat_Decal" (`KismetMathLibrary.MakeVector` _returnvalue _returnvalue _returnvalue) OtherComp "None" (`KismetMathLibrary.InverseTransformLocation` _returnvalue_2 HitLocation) (`KismetMathLibrary.InverseTransformRotation` _returnvalue_2 (`SceneComponent.K2_GetComponentRotation` MyComp)) "KeepRelativeOffset" 10.0))))

(fn `ComputeExiteLocation`
  (params (Hit :type "HitResult Structure (by ref)") (A :type "Vector Structure"))
  (returns (ExitLocation :type "Vector Structure") (ResultFound :type Boolean)))

(fn `UserConstructionScript`
  (`parent.UserConstructionScript`))