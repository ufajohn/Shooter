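; Knife melee weapon that deals point damage to what it hits in front of the player.
; It can be used whenever it is not frozen by its use rate.
; When the parent use succeeds, a sphere trace runs from the player's FreeCamera along the owner's forward vector for the Radius distance, ignoring the instigator.
; The trace's hit result feeds point damage credited to the instigator's controller.
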(fn `AbleToUseWeapon`
  (returns (Out :type Boolean))
  (return (not (`self.UseFreezedByRate`))))

(fn `Damage_0`
  (returns (hit :type "HitResult Structure"))
  (bind _asbp_player_character (cast `/Game/Blueprints/Characters/BP_PlayerCharacter` (`self.GetInstigator`))
    (:`then`
      (bind _returnvalue (`SceneComponent.K2_GetComponentLocation` (`/Game/Blueprints/Characters/BP_PlayerCharacter.FreeCamera` _asbp_player_character)))
      (bind _outhit (`KismetSystemLibrary.SphereTraceSingleForObjects` _returnvalue (+ _returnvalue (* (`self.GetActorForwardVector` (`self.GetOwner`)) (`self.radius`))) 30.0 (`|MakeArray` "ObjectTypeQuery1" "ObjectTypeQuery2" "ObjectTypeQuery3" :!type "EObjectTypeQuery Enum") false (`|MakeArray` (`self.GetInstigator`) :!type "Actor Object Reference")))
      (return _outhit))
    (:`CastFailed`
      (return))))

(fn `UserConstructionScript`
  (`parent.UserConstructionScript`))

(fn `UseWeapon`
  (params (SpawnTransform :type "Transform Structure"))
  (returns (Used :type Boolean))
  (bind _used (`parent.UseWeapon` (struct)))
  (if _used
    (bind _hit (`self.Damage_0`))
    (bind (_bblockinghit _binitialoverlap _time _distance _location _impactpoint _normal _impactnormal _physmat _hitactor _hitcomponent _hitbonename _hititem _faceindex _tracestart _traceend) (`GameplayStatics.BreakHitResult` _hit))
    (`GameplayStatics.ApplyPointDamage` _hitactor (`self.damage`) (`KismetMathLibrary.GetDirectionUnitVector` _traceend _tracestart) _hit (`self.GetInstigatorController`) self)
    (return true)
    (else
      (return false))))